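; BP_BuffComponent tracks the buffs held by the boss and Peppy and shows their icons on the battle HUD.
; Add functions store the buff name and create an icon widget with a texture from BuffTable, while Update functions recreate icons from the stored lists.
; Boss icons fill one row and Peppy's wrap every five columns.
; UpdatePeppyBuffUI targets the boss panel, unlike AddPeppyBuffUI.
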(fn `AddBossBuffUI`
  (params (BuffType :type "EBuffType Enum" :default "AttackIncrease"))
  (`self.Set BP_BattleHUD`)
  (bind _returnvalue (`self.BuffTypeToString` BuffType))
  (bind _returnvalue_2 (`KismetArrayLibrary.Array_Add` (`self.HasBossBuff`) _returnvalue))
  (`self.Create And Add Buff Icon In Panel` _returnvalue 0 _returnvalue_2 (`/Game/Blueprints/UMG/BP_BattleHUD.UniformGridPanel_BossBuff` (`self.BP_BattleHUD`))))

(fn `AddPeppyBuffUI`
  (params (BuffType :type "EBuffType Enum" :default "AttackIncrease"))
  (`self.Set BP_BattleHUD`)
  (bind _returnvalue (`self.BuffTypeToString` BuffType))
  (bind _returnvalue_2 (`KismetArrayLibrary.Array_Add` (`self.HasPeppyBuff`) _returnvalue))
  (`self.Create And Add Buff Icon In Panel` _returnvalue (- 1 (/ _returnvalue_2 5)) (mod _returnvalue_2 5) (`/Game/Blueprints/UMG/BP_BattleHUD.UniformGridPanel_PeppyBuff` (`self.BP_BattleHUD`)))
  (`KismetSystemLibrary.PrintString` "Hello"))

(fn `Create And Add Buff Icon In Panel`
  (params (`Buff Name` :type String) (Row :type Integer) (Column :type Integer) (`Uniform Grid Panel Ref` :type "UniformGridPanel Object Reference"))
  (bind _returnvalue (`|CreateWidget` "/Game/Blueprints/UMG/BP_BuffIconForm.BP_BuffIconForm_C"))
  (`UserWidget.AddToViewport` _returnvalue 0)
  (bind _newparam (`self.Find Buff Icon By Name` `Buff Name`))
  (`Image.SetBrushFromTexture` (`/Game/Blueprints/UMG/BP_BuffIconForm.Image_Icon` _returnvalue) _newparam false)
  (`UniformGridPanel.AddChildToUniformGrid` (`local.Uniform Grid Panel Ref`) _returnvalue (`local.Row`) (`local.Column`)))

(fn `Find Buff Icon By Name`
  (params (BuffName :type String))
  (returns (NewParam :type "Texture2D Object Reference"))
  (bind _returnvalue (`|GetDataTableRow` "/Game/Assets/DataTable/BuffTable.BuffTable" (`KismetStringLibrary.Conv_StringToName` BuffName))
    (:`then`
      (return (`.BuffIcon` (break `BuffTable` _returnvalue))))))

(fn `Set BP_BattleHUD`
  (bind _foundwidgets (`WidgetBlueprintLibrary.GetAllWidgetsOfClass` "/Game/Blueprints/UMG/BP_BattleHUD.BP_BattleHUD_C"))
  (bind _output (`|GetArrayItem` _foundwidgets))
  (`/Engine/EditorBlueprintResources/StandardMacros.IsValid` _output
    (:`Is Valid`
      (set `self.BP_BattleHUD` _output))))

(fn `UpdateBossBuffUI`
  (`self.Set BP_BattleHUD`)
  (for (_array_element _array_index) (`self.HasBossBuff`)
    (`self.Create And Add Buff Icon In Panel` _array_element 0 _array_index (`/Game/Blueprints/UMG/BP_BattleHUD.UniformGridPanel_BossBuff` (`self.BP_BattleHUD`)))))

(fn `UpdatePeppyBuffUI`
  (`self.Set BP_BattleHUD`)
  (for (_array_element _array_index) (`self.HasPeppyBuff`)
    (`self.Create And Add Buff Icon In Panel` _array_element (- 1 (/ _array_index 5)) (mod _array_index 5) (`/Game/Blueprints/UMG/BP_BattleHUD.UniformGridPanel_BossBuff` (`self.BP_BattleHUD`)))))