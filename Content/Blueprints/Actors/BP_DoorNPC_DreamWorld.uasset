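; Interactable door NPC for the dream world that sends the player to the hub level.
; On BeginPlay it labels its interaction popup widget as a gate with an enter prompt and binds the button click.
; Interaction events toggle the CanInteraction flag and popup visibility.
; Clicking plays a sound at a hardcoded location, waits briefly, then opens LV_HubWorld; hover-outline logic is left unconnected.
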(event `BP Initialization 이벤트`
  ;[1 1 1] Init setting NPC
  (set `self.Mesh` (`self.HERBWORLDmodelling_house_door`)))

(event `self.ReceiveBeginPlay`
  ;[1 1 1] Set widget text block to its NPC name
  (`self.BP Initialization 이벤트`)
  (bind _asbp_interaction_popup (cast `/Game/Blueprints/UMG/BP_InteractionPopup` (`WidgetComponent.GetUserWidgetObject` (`self.Widget`))))
  (bind _output_get (set `self.InteractionUI` _asbp_interaction_popup))
  (`/Game/Blueprints/UMG/BP_InteractionPopup.Set NPC Interaction text` _output_get "대문" "입장하기")
  (add `Button.OnClicked` (`/Game/Blueprints/UMG/BP_InteractionPopup.버튼_상호작용` (`self.InteractionUI`)) (delegate `Interaction Button Click 이벤트`)))

(event `Interaction Button Click 이벤트`
  (`GameplayStatics.SpawnSoundAtLocation` null (894.0 1099.0 449.0) (struct) 1.0 1.0 0.0 null null false)
  (`KismetSystemLibrary.Delay` 1.0)
  (`GameplayStatics.OpenLevelBySoftObjectPtr` "/Game/Levels/LV_HubWorld.LV_HubWorld"))

(event `self.SetCanInteraction`
  ;[1 1 1] Check overlap to interaction capsule of Peppy : Show and hide interaction UI
  (set `NPCComponent.CanInteraction` true (`self.NPC`))
  (`SceneComponent.SetHiddenInGame` (`self.Widget`) false false))

(event `self.SetCannotInteraction`
  ;[1 1 1] Check overlap to interaction capsule of Peppy : Show and hide interaction UI
  (set `NPCComponent.CanInteraction` false (`self.NPC`))
  (`SceneComponent.SetHiddenInGame` (`self.Widget`) true false))

(fn `UserConstructionScript`)