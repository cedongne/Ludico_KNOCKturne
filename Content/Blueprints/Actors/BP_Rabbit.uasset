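; BP_Rabbit is a rabbit NPC that signals when the player can interact with it.
; On BeginPlay it sets its widget component's InteractionPopup name to "토끼" (rabbit).
; Interaction events, meant for overlap with Peppy's capsule, toggle CanInteraction and the popup, using custom depth to highlight the mesh if hovered.
; The click event is empty, and the voice-and-"Hello" greeting is disconnected, so it never runs.
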(event `self.ReceiveBeginPlay`
  ;[1 1 1] Set widget text block to its NPC name
  (bind _asinteraction_popup (cast `/Game/Blueprints/UMG/InteractionPopup` (`WidgetComponent.GetUserWidgetObject` (`self.Widget`))))
  (bind _output_get (set `self.Name` "토끼"))
  (`/Game/Blueprints/UMG/InteractionPopup.SetName` _asinteraction_popup _output_get))

(event `self.SetCanInteraction`
  ;[1 1 1] Check overlap to interaction capsule of Peppy : Show and hide interaction UI
  (set `NPCComponent.CanInteraction` true (`self.NPC`))
  (`SceneComponent.SetHiddenInGame` (`self.Widget`) false false)
  (if (`self.IsHoverMouse`)
    (`PrimitiveComponent.SetRenderCustomDepth` (`self.herbworld_rabbitnpc`) true)))

(event `self.SetCannotInteraction`
  ;[1 1 1] Check overlap to interaction capsule of Peppy : Show and hide interaction UI
  (set `NPCComponent.CanInteraction` false (`self.NPC`))
  (`SceneComponent.SetHiddenInGame` (`self.Widget`) true false)
  (`PrimitiveComponent.SetRenderCustomDepth` (`self.herbworld_rabbitnpc`) false))

(event `self.ReceiveActorOnClicked`
  (params (ButtonPressed :type "Key Structure")))

(fn `UserConstructionScript`)