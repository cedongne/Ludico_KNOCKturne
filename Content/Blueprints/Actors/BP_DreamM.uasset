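; BP_DreamM is the rabbit NPC that offers Peppy random talk or dream-fragment interpretation.
; Interaction events toggle its popup, choosing the talk icon by whether Peppy holds dream fragments.
; Tick polls E while Peppy overlaps it, moves the camera, then starts random talk or opens a two-option BP_Dialogue.
; Branching reads UI state: brush textures identify the talk type and selected option, which triggers the matching dialogue call.
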(event `BP Initialization 이벤트`
  ;[1 1 1] Init setting NPC
  (set `self.Mesh` (`self.npc_dreamM`)))

(event `self.ReceiveBeginPlay`
  ;[1 1 1] Set widget text block to its NPC name
  (`self.BP Initialization 이벤트`)
  (bind _asbp_interaction_popup (cast `/Game/Blueprints/UMG/BP_InteractionPopup` (`WidgetComponent.GetUserWidgetObject` (`self.Widget`))))
  (bind _output_get (set `self.InteractionUI` _asbp_interaction_popup))
  (`/Game/Blueprints/UMG/BP_InteractionPopup.Set NPC Interaction text` _output_get "토끼" "대화하기"))

(event `self.SetCanInteraction`
  (bind _image_interaction (`/Game/Blueprints/UMG/BP_InteractionPopup.Image_interaction` (`self.InteractionUI`)))
  ;[1 1 1] Check overlap to interaction capsule of Peppy : Show and hide interaction UI
  (bind _returnvalue (`GameplayStatics.GetActorOfClass` "/Game/Blueprints/Actors/BP_Peppy.BP_Peppy_C"))
  (if (not (`/Game/Blueprints/Actors/BP_Peppy.isTalking` _returnvalue))
    (set `NPCComponent.CanInteraction` true (`self.NPC`))
    (`SceneComponent.SetHiddenInGame` (`self.Widget`) false false)
    (bind _outactors (`GameplayStatics.GetAllActorsOfClass` "/Game/Blueprints/Actors/BP_Peppy.BP_Peppy_C"))
    (if (> (`/Game/Blueprints/Actors/BP_Peppy.DreanFragment Count` (`|GetArrayItem` _outactors)) 0)
      (`Image.SetBrushFromTexture` _image_interaction "/Game/Assets/Art_UI/HubWorld/UI_hubworld_talk_v2.UI_hubworld_talk_v2" false)
      (else
        (`Image.SetBrushFromTexture` _image_interaction "/Game/Assets/Art_UI/HubWorld/UI_hubworld_talk_v1.UI_hubworld_talk_v1" false)))))

(event `self.SetCannotInteraction`
  ;[1 1 1] Check overlap to interaction capsule of Peppy : Show and hide interaction UI
  (set `NPCComponent.CanInteraction` false (`self.NPC`))
  (`SceneComponent.SetHiddenInGame` (`self.Widget`) true false))

(event `SelectDialogue`
  (if (`|EnumEquality` (`Widget.GetVisibility` (`/Game/Blueprints/UMG/BP_Dialogue.Image_Dialogue_Select_1` (`self.BP_Dialogue`))) "Visible")
    (`Widget.SetVisibility` (`/Game/Blueprints/UMG/BP_Dialogue.Image_Dialogue_Select_1` (`self.BP_Dialogue`)) "Hidden")
    (`Widget.SetVisibility` (`/Game/Blueprints/UMG/BP_Dialogue.Image_Dialogue_Select_2` (`self.BP_Dialogue`)) "Hidden")
    (`Widget.SetVisibility` (`/Game/Blueprints/UMG/BP_Dialogue.TextBlock_Dialogue_Select_1` (`self.BP_Dialogue`)) "Hidden")
    (`Widget.SetVisibility` (`/Game/Blueprints/UMG/BP_Dialogue.TextBlock_Dialogue_Select_2` (`self.BP_Dialogue`)) "Hidden")
    (`Widget.SetVisibility` (`/Game/Blueprints/UMG/BP_Dialogue.RichTextBlock_Dialogue` (`self.BP_Dialogue`)) "Hidden")
    (if (== (`WidgetBlueprintLibrary.GetBrushResource` (`Image.Brush` (`/Game/Blueprints/UMG/BP_Dialogue.Image_Dialogue_Select_1` (`self.BP_Dialogue`)))) "/Game/Assets/Art_UI/Dialog/UI_dia_DreamFragments/icon_dia_select_yes_32_32.icon_dia_select_yes_32_32")
      (`self.DreamM_DreamFragment`)
      (`Widget.SetVisibility` (`/Game/Blueprints/UMG/BP_Dialogue.Image_Npc` (`self.BP_Dialogue`)) "Visible" :!label _label)
      (`Widget.SetVisibility` (`/Game/Blueprints/UMG/BP_Dialogue.Overlay_NpcName` (`self.BP_Dialogue`)) "Visible")
      (set `self.BeforeSelectingDialogue` false)
      (elif (== (`WidgetBlueprintLibrary.GetBrushResource` (`Image.Brush` (`/Game/Blueprints/UMG/BP_Dialogue.Image_Dialogue_Select_2` (`self.BP_Dialogue`)))) "/Game/Assets/Art_UI/Dialog/UI_dia_DreamFragments/icon_dia_select_yes_32_32.icon_dia_select_yes_32_32")
        (`self.DreamM_RandomTalk`)
        (goto _label)))))

(event `self.ReceiveTick`
  (params (DeltaSeconds :type "Float (single-precision)"))
  (bind _bp_dialogue (`self.BP_Dialogue`))
  (bind _asbp_peppy (cast `/Game/Blueprints/Actors/BP_Peppy` (`GameplayStatics.GetPlayerPawn` 0)))
  (if (== (`/Game/Blueprints/Actors/BP_Peppy.OverlappedActor` _asbp_peppy) self)
    (bind _returnvalue (`GameplayStatics.GetActorOfClass` "/Game/Blueprints/Actors/BP_Peppy.BP_Peppy_C"))
    (if (`/Game/Blueprints/Actors/BP_Peppy.isTalking` _returnvalue)
      _
      (elif (`PlayerController.WasInputKeyJustPressed` (`GameplayStatics.GetPlayerController` 0) "E")
        (if (`self.BeforeSelectingDialogue`)
          (`self.SelectDialogue`)
          (else
            (`GameplayStatics.SpawnSoundAtLocation` null (0.0 0.0 0.0) (struct) 1.0 1.0 0.0 null null)
            (bind _asbp_peppy_2 (cast `/Game/Blueprints/Actors/BP_Peppy` (`GameplayStatics.GetPlayerPawn` 0)))
            (`/Game/Blueprints/Actors/BP_Peppy.Interaction Camera Move 이벤트` _asbp_peppy_2 self)
            (if (== (`WidgetBlueprintLibrary.GetBrushResource` (`Image.Brush` (`/Game/Blueprints/UMG/BP_InteractionPopup.Image_interaction` (`self.InteractionUI`)))) "/Game/Assets/Art_UI/HubWorld/UI_hubworld_talk_v1.UI_hubworld_talk_v1")
              (set `self.BeforeSelectingDialogue` false)
              (`self.DreamM_RandomTalk`)
              (else
                (bind _returnvalue_2 (`|CreateWidget` "/Game/Blueprints/UMG/BP_Dialogue.BP_Dialogue_C" :!label _label_2))
                (bind _output_get (set `self.BP_Dialogue` _returnvalue_2))
                (`UserWidget.AddToViewport` _returnvalue_2 0)
                (`UserWidget.AddToViewport` _output_get 0)
                (set `self.BeforeSelectingDialogue` true :!label _label_3)
                (`Widget.SetVisibility` (`/Game/Blueprints/UMG/BP_Dialogue.Image_Dialogue_Select_1` _bp_dialogue) "Visible")
                (`Widget.SetVisibility` (`/Game/Blueprints/UMG/BP_Dialogue.Image_Dialogue_Select_2` _bp_dialogue) "Visible")
                (`Widget.SetVisibility` (`/Game/Blueprints/UMG/BP_Dialogue.TextBlock_Dialogue_Select_1` _bp_dialogue) "Visible")
                (`Widget.SetVisibility` (`/Game/Blueprints/UMG/BP_Dialogue.TextBlock_Dialogue_Select_2` _bp_dialogue) "Visible")
                (`Widget.SetVisibility` (`/Game/Blueprints/UMG/BP_Dialogue.Image_Npc` (`self.BP_Dialogue`)) "Hidden")
                (`Widget.SetVisibility` (`/Game/Blueprints/UMG/BP_Dialogue.Overlay_NpcName` (`self.BP_Dialogue`)) "Hidden")
                (`Image.SetOpacity` (`/Game/Blueprints/UMG/BP_Dialogue.Image_CutScene` (`self.BP_Dialogue`)) 0.0)
                (`TextBlock.SetText` (`/Game/Blueprints/UMG/BP_Dialogue.Text_PeppyName` (`self.BP_Dialogue`)) "페피")))))))))

(event `Create Widget and Start Select Dialogue`
  (goto _label_2))

(event `Start Select Dialogue`
  (goto _label_3))

(fn `UserConstructionScript`)