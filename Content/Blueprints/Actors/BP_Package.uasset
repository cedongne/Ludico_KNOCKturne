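; BP_Package is an interactable package actor that opens the BP_BeforeBattleSkill screen when the player interacts with it.
; On BeginPlay it caches its interaction popup widget and binds to BP_PeppyController's start-interaction event.
; That event creates the screen only if BP_Peppy's OverlappedActor is this package.
; Separate events toggle the CanInteraction flag and popup visibility; key-polling and hover-outline logic remain unconnected.
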(event `BP Initialization 이벤트`
  ;[1 1 1] Init setting NPC
  (set `self.Mesh` (`self.hubworld_package2`)))

(event `self.ReceiveBeginPlay`
  ;[1 1 1] Set widget text block to its NPC name
  (`self.BP Initialization 이벤트`)
  (bind _asbp_interaction_popup (cast `/Game/Blueprints/UMG/BP_InteractionPopup` (`WidgetComponent.GetUserWidgetObject` (`self.Widget`))))
  (set `self.InteractionUI` _asbp_interaction_popup)
  (bind _asbp_peppy_controller (cast `/Game/Blueprints/GameModes/BP_PeppyController` (`GameplayStatics.GetPlayerController` 0)))
  (add `/Game/Blueprints/GameModes/BP_PeppyController.Start Interaction` _asbp_peppy_controller (delegate `Package Start Interaction`)))

(event `Package Start Interaction`
  (bind _asbp_peppy (cast `/Game/Blueprints/Actors/BP_Peppy` (`GameplayStatics.GetPlayerPawn` 0)))
  (if (== (`/Game/Blueprints/Actors/BP_Peppy.OverlappedActor` _asbp_peppy) self)
    (bind _returnvalue (`|CreateWidget` "/Game/Blueprints/UMG/BP_BeforeBattleSkill.BP_BeforeBattleSkill_C"))
    (`UserWidget.AddToViewport` _returnvalue 0)))

(event `self.SetCanInteraction`
  ;[1 1 1] Check overlap to interaction capsule of Peppy : Show and hide interaction UI
  (set `NPCComponent.CanInteraction` true (`self.NPC`))
  (`SceneComponent.SetHiddenInGame` (`self.Widget`) false false))

(event `self.SetCannotInteraction`
  ;[1 1 1] Check overlap to interaction capsule of Peppy : Show and hide interaction UI
  (set `NPCComponent.CanInteraction` false (`self.NPC`))
  (`SceneComponent.SetHiddenInGame` (`self.Widget`) true false))

(event `self.ReceiveTick`
  (params (DeltaSeconds :type "Float (single-precision)")))

(fn `UserConstructionScript`)