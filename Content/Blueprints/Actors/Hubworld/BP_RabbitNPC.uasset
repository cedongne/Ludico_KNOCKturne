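; Rabbit NPC actor for the hubworld that offers Peppy a talk interaction.
; On BeginPlay it sets up its mesh, caches the interaction popup widget and binds RabbitStartTalk to the Peppy controller's start-interaction event.
; Can/cannot-interaction events toggle the NPC flag and popup visibility, while talk events play sounds or call rabbit talk hooks.
; An unconnected branch holds overlap-checked camera movement and random talk.
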(event `BP Initialization 이벤트`
  ;[1 1 1] Init setting NPC
  (set `self.Mesh` (`self.herbworld_rabbitnpc`)))

(event `self.ReceiveBeginPlay`
  ;[1 1 1] Set widget text block to its NPC name
  (`self.BP Initialization 이벤트`)
  (bind _asbp_interaction_popup (cast `/Game/Blueprints/UMG/BP_InteractionPopup` (`WidgetComponent.GetUserWidgetObject` (`self.Widget`))))
  (set `self.InteractionUI` _asbp_interaction_popup)
  (bind _asbp_peppy_controller (cast `/Game/Blueprints/GameModes/BP_PeppyController` (`GameplayStatics.GetPlayerController` 0)))
  (add `/Game/Blueprints/GameModes/BP_PeppyController.Start Interaction` _asbp_peppy_controller (delegate `Rabbit Start Talk`)))

(event `self.RabbitRandomTalk`
  (`self.Rabbit RandomTalk`))

(event `Rabbit Start Talk`
  (`GameplayStatics.SpawnSoundAtLocation` null (0.0 0.0 0.0) (struct) 1.0 1.0 0.0 null null)
  (`self.RabbitStartTalk`))

(event `self.SetCanInteraction`
  ;[1 1 1] Check overlap to interaction capsule of Peppy : Show and hide interaction UI
  (set `NPCComponent.CanInteraction` true (`self.NPC`))
  (`SceneComponent.SetHiddenInGame` (`self.Widget`) false false))

(event `self.SetCannotInteraction`
  ;[1 1 1] Check overlap to interaction capsule of Peppy : Show and hide interaction UI
  (set `NPCComponent.CanInteraction` false (`self.NPC`))
  (`SceneComponent.SetHiddenInGame` (`self.Widget`) true false))

(fn `UserConstructionScript`)