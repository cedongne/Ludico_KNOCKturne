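; BP_DoorNPC_Hubworld is an interactable hubworld door that sends the player into the battle level, LV_Battle.
; On BeginPlay it caches its interaction popup widget and binds DoorStartInteraction to BP_PeppyController's interaction event.
; That handler confirms Peppy is overlapping this door, plays a sound at a hardcoded location, then opens the level after a short delay.
; SetCanInteraction and SetCannotInteraction toggle the NPC's interactable flag and popup visibility.
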(event `BP Initialization 이벤트`
  ;[1 1 1] Init setting NPC
  (set `self.Mesh` (`self.HERBWORLDmodelling_house_door`)))

(event `self.ReceiveBeginPlay`
  ;[1 1 1] Set widget text block to its NPC name
  (`self.BP Initialization 이벤트`)
  (bind _asbp_interaction_popup (cast `/Game/Blueprints/UMG/BP_InteractionPopup` (`WidgetComponent.GetUserWidgetObject` (`self.Widget`))))
  (set `self.InteractionUI` _asbp_interaction_popup)
  (bind _asbp_peppy_controller (cast `/Game/Blueprints/GameModes/BP_PeppyController` (`GameplayStatics.GetPlayerController` 0)))
  (add `/Game/Blueprints/GameModes/BP_PeppyController.Start Interaction` _asbp_peppy_controller (delegate `Door Start Interaction`)))

(event `Door Start Interaction`
  (bind _asbp_peppy (cast `/Game/Blueprints/Actors/BP_Peppy` (`GameplayStatics.GetPlayerPawn` 0)))
  (if (== (`Peppy.OverlappedActor` _asbp_peppy) self)
    (if (`/Game/Blueprints/Actors/BP_Peppy.isOverlapped` _asbp_peppy)
      (`GameplayStatics.SpawnSoundAtLocation` null (894.0 1099.0 449.0) (struct) 1.0 1.0 0.0 null null false)
      (`KismetSystemLibrary.Delay` 1.0)
      (`GameplayStatics.OpenLevelBySoftObjectPtr` "/Game/Levels/LV_Battle.LV_Battle"))))

(event `self.SetCanInteraction`
  ;[1 1 1] Check overlap to interaction capsule of Peppy : Show and hide interaction UI
  (set `NPCComponent.CanInteraction` true (`self.NPC`))
  (`SceneComponent.SetHiddenInGame` (`self.Widget`) false false))

(event `self.SetCannotInteraction`
  ;[1 1 1] Check overlap to interaction capsule of Peppy : Show and hide interaction UI
  (set `NPCComponent.CanInteraction` false (`self.NPC`))
  (`SceneComponent.SetHiddenInGame` (`self.Widget`) true false))

(fn `UserConstructionScript`)