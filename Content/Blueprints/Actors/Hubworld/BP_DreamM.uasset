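; Hubworld NPC DreamM, whom Peppy can talk to through an interaction popup.
; BeginPlay caches the popup and binds talk start to BP_PeppyController's interaction event.
; SetCanInteraction shows the popup, choosing a mission or talk icon from the game state's battle-clear flag and dream fragment count.
; Talk events forward to dialogue calls defined outside this graph; the icon-based branching and choice-selection logic here is disconnected.
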(event `BP Initialization 이벤트`
  ;[1 1 1] Init setting NPC
  (set `self.Mesh` null))

(event `self.ReceiveBeginPlay`
  ;[1 1 1] Set widget text block to its NPC name
  (`self.BP Initialization 이벤트`)
  (bind _asbp_interaction_popup (cast `/Game/Blueprints/UMG/BP_InteractionPopup` (`WidgetComponent.GetUserWidgetObject` (`self.Widget`))))
  (set `self.InteractionUI` _asbp_interaction_popup)
  (bind _asbp_peppy_controller (cast `/Game/Blueprints/GameModes/BP_PeppyController` (`GameplayStatics.GetPlayerController` 0)))
  (add `/Game/Blueprints/GameModes/BP_PeppyController.Start Interaction` _asbp_peppy_controller (delegate `DreamM Start Talk`)))

(event `self.SetPeppyName`
  (bind _foundwidgets (`WidgetBlueprintLibrary.GetAllWidgetsOfClass` "/Game/Blueprints/UMG/BP_Dialogue.BP_Dialogue_C"))
  (`TextBlock.SetText` (`/Game/Blueprints/UMG/BP_Dialogue.Text_PeppyName` (`|GetArrayItem` _foundwidgets)) "페피"))

(event `DreamM Start Talk`
  (`GameplayStatics.SpawnSoundAtLocation` null (0.0 0.0 0.0) (struct) 1.0 1.0 0.0 null null)
  (`self.DreamMStartTalk`))

(event `self.DreamMAfterBattleTalk`
  (`self.DreamM_AfterBattleTalk`))

(event `self.DreamMRandomTalk`
  (`self.DreamM_RandomTalk`))

(event `self.DreamMDreamFragment`
  (`self.DreamM_DreamFragment`))

(event `self.SetCanInteraction`
  (bind _image_interaction (`/Game/Blueprints/UMG/BP_InteractionPopup.Image_interaction` (`self.InteractionUI`)))
  ;[1 1 1] Check overlap to interaction capsule of Peppy : Show and hide interaction UI
  (set `NPCComponent.CanInteraction` true (`self.NPC`))
  (`SceneComponent.SetHiddenInGame` (`self.Widget`) false false)
  (bind _asknockturne_game_state (cast `KNOCKturneGameState` (`GameplayStatics.GetGameState`)))
  (if (`KNOCKturneGameState.RightafterBattleClear` _asknockturne_game_state)
    (`Image.SetBrushFromTexture` (`/Game/Blueprints/UMG/BP_InteractionPopup.Image_interaction` (`self.InteractionUI`)) "/Game/Assets/Art_UI/HubWorld/UI_icon_mission.UI_icon_mission" false)
    (else
      (bind _asknockturne_game_state_2 (cast `KNOCKturneGameState` (`GameplayStatics.GetGameState`)))
      (if (> (`KNOCKturneGameState.DreamFragmentCount` _asknockturne_game_state_2) 0)
        (`Image.SetBrushFromTexture` _image_interaction "/Game/Assets/Art_UI/HubWorld/UI_hubworld_talk_v2.UI_hubworld_talk_v2" false)
        (else
          (`Image.SetBrushFromTexture` _image_interaction "/Game/Assets/Art_UI/HubWorld/UI_hubworld_talk_v1.UI_hubworld_talk_v1" false))))))

(event `self.SetCannotInteraction`
  ;[1 1 1] Check overlap to interaction capsule of Peppy : Show and hide interaction UI
  (set `NPCComponent.CanInteraction` false (`self.NPC`))
  (`SceneComponent.SetHiddenInGame` (`self.Widget`) true false))

(event `SelectDialogueEvent`)

(fn `UserConstructionScript`)