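; BP_NPC is a clickable NPC actor that shows an outline and interaction widget when it can be interacted with.
; SetCanInteraction and SetCannotInteraction, meant for overlaps with Peppy's interaction capsule, set the flag and toggle the widget.
; Cursor hover combines with that flag to toggle Custom Depth on the skeletal mesh for the outline.
; Clicking while interaction is allowed plays a test voice cue and prints a placeholder greeting.
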(event `self.ReceiveActorBeginCursorOver`
  ;[1 1 1] Cursor hover Events : Show and hide outline
  (set `self.IsHoverMouse` true)
  (if (`NPCComponent.CanInteraction` (`self.NPC`))
    (`PrimitiveComponent.SetRenderCustomDepth` (`self.SkeletalMesh`) true)))

(event `self.ReceiveActorEndCursorOver`
  ;[1 1 1] Cursor hover Events : Show and hide outline
  (set `self.IsHoverMouse` false)
  (if (`NPCComponent.CanInteraction` (`self.NPC`))
    _
    (else
      _))
  (`PrimitiveComponent.SetRenderCustomDepth` (`self.SkeletalMesh`) false))

(event `SetCanInteraction`
  ;[1 1 1] Check overlap to interaction capsule of Peppy : Show and hide interaction UI
  (set `NPCComponent.CanInteraction` true (`self.NPC`))
  (`SceneComponent.SetHiddenInGame` (`self.Widget`) false false)
  (if (`self.IsHoverMouse`)
    (`PrimitiveComponent.SetRenderCustomDepth` (`self.SkeletalMesh`) true)))

(event `SetCannotInteraction`
  ;[1 1 1] Check overlap to interaction capsule of Peppy : Show and hide interaction UI
  (set `NPCComponent.CanInteraction` false (`self.NPC`))
  (`SceneComponent.SetHiddenInGame` (`self.Widget`) true false)
  (`PrimitiveComponent.SetRenderCustomDepth` (`self.SkeletalMesh`) false))

(event `self.ReceiveActorOnClicked`
  (params (ButtonPressed :type "Key Structure"))
  (if (`NPCComponent.CanInteraction` (`self.NPC`))
    (`GameplayStatics.SpawnSoundAtLocation` "/Game/Assets/Sounds/Voice/Voice_NPCTest_Cue.Voice_NPCTest_Cue" (0.0 0.0 0.0) (struct) 1.0 1.0 0.0 null null)
    (`KismetSystemLibrary.PrintText` "Hello")))

(fn `UserConstructionScript`)