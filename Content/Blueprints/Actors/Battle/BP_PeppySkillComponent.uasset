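; Battle component that handles Peppy's special skill, spending energy and showing its cooldown on the battle HUD.
; UseSpecialSkill resolves the skill row from the HUD's specialty icon name via BattleManagerSystem and reads SpecialSkillTable.
; Energy is deducted only when the cost exceeds current energy (an apparently inverted check), then UsingSpecialSkill updates icons and starts the HUD timer.
; SpecialSkillAfterOneTurn sets a cooldown display, but its call is unwired.
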(event `self.ReceiveBeginPlay`
  (bind _foundwidgets (`WidgetBlueprintLibrary.GetAllWidgetsOfClass` "/Game/Blueprints/UMG/BP_BattleHUD.BP_BattleHUD_C"))
  (set `self.BP_BattleHUD` (`|GetArrayItem` _foundwidgets)))

(fn `Special Skill After One Turn`
  (params (`Timer Value` :type Integer))
  (`Widget.SetVisibility` (`/Game/Blueprints/UMG/BP_BattleHUD.Image_Specialty_Active` (`self.BP_BattleHUD`)) "Hidden")
  (`Widget.SetVisibility` (`/Game/Blueprints/UMG/BP_BattleHUD.TextBlock_SpecialtyKey` (`self.BP_BattleHUD`)) "Hidden")
  (`Widget.SetVisibility` (`/Game/Blueprints/UMG/BP_BattleHUD.Image_Opacity60` (`self.BP_BattleHUD`)) "Visible")
  (set `/Game/Blueprints/UMG/BP_BattleHUD.TimerValue` (`local.Timer Value`) (`self.BP_BattleHUD`))
  (`Widget.SetVisibility` (`/Game/Blueprints/UMG/BP_BattleHUD.TextBlock_Specialty_Timer` (`self.BP_BattleHUD`)) "Visible"))

(fn `Use Special Skill`
  (bind `_현재에너지` (`/Game/Blueprints/UMG/BP_BattleHUD.현재에너지` (`self.BP_BattleHUD`)))
  (bind _returnvalue (`BattleManagerSystem.FindSpecialtyRow` (subsystem `BattleManagerSystem`) (`KismetSystemLibrary.GetObjectName` (`WidgetBlueprintLibrary.GetBrushResource` (`Image.Brush` (`/Game/Blueprints/UMG/BP_BattleHUD.Image_Specialty` (`self.BP_BattleHUD`)))))))
  (bind _outrownames (`DataTableFunctionLibrary.GetDataTableRowNames` "/Game/Assets/DataTable/SpecialSkillTable.SpecialSkillTable"))
  (bind _returnvalue_2 (`|GetDataTableRow` "/Game/Assets/DataTable/SpecialSkillTable.SpecialSkillTable" (`|GetArrayItem` _outrownames _returnvalue))
    (:`then`
      (bind (_skill_index _probability_1 _specialskill_target _value1n _value1m _value1t _buffcode _energycost _cooltime) (break `SpecialSkillData` _returnvalue_2))
      (if (> _energycost `_현재에너지`)
        (set `/Game/Blueprints/UMG/BP_BattleHUD.현재에너지` (- `_현재에너지` _energycost) (`self.BP_BattleHUD`))
        (`self.Using Special Skill` _cooltime)))))

(fn `Using Special Skill`
  (params (`Timer Value` :type Integer))
  (bind _timer_value (`local.Timer Value`))
  (`Widget.SetVisibility` (`/Game/Blueprints/UMG/BP_BattleHUD.Image_Specialty_Active` (`self.BP_BattleHUD`)) "Visible")
  (`Widget.SetVisibility` (`/Game/Blueprints/UMG/BP_BattleHUD.TextBlock_SpecialtyKey` (`self.BP_BattleHUD`)) "Hidden")
  (`Widget.SetVisibility` (`/Game/Blueprints/UMG/BP_BattleHUD.Image_Opacity60` (`self.BP_BattleHUD`)) "Visible")
  (if (> _timer_value 0)
    (set `/Game/Blueprints/UMG/BP_BattleHUD.TimerValue` _timer_value (`self.BP_BattleHUD`))
    (`Widget.SetVisibility` (`/Game/Blueprints/UMG/BP_BattleHUD.TextBlock_Specialty_Timer` (`self.BP_BattleHUD`)) "Visible")
    (`/Game/Blueprints/UMG/BP_BattleHUD.Timer` (`self.BP_BattleHUD`))))