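; BP_FootholdSpawner is a battle actor that places pooled foothold actors at random spots in the battle area.
; Its Stamp event, fired on BeginPlay, alternates between the first two KNOCKturneObjectPool entries, moves the selected one to a random point in a hard-coded flat box and unhides it.
; It reuses existing actors instead of spawning new ones, and never hides the previous foothold itself.
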(event `self.ReceiveBeginPlay`
  (`self.Stamp`))

(event `Stamp`
  (bind _output_get (set `self.CurrentFootholdIndex` (mod (+ (`self.CurrentFootholdIndex`) 1) 2)))
  (bind _output (`|GetArrayItem` (`KNOCKturneObjectPool.ObjectPool` (`self.KNOCKturneObjectPool`)) _output_get))
  (`self.K2_SetActorLocation` _output (`KismetMathLibrary.RandomPointInBoundingBox` (751.0 774.0 -90.0) (400.0 400.0 0.0)) false false)
  (`self.SetActorHiddenInGame` _output false))

(fn `UserConstructionScript`)