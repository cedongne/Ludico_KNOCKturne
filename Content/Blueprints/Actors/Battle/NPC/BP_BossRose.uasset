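; BP_BossRose is a battle boss that spawns random skill actors during its turn.
; Turn start and end toggle Tick, whose timer fires immediately, then about every five seconds.
; Each firing draws class and transform from random keys in the battle table manager's BossSkillSpawnDataMap.
; BeginPlay caches the energy spawner, but the SpawnEnergy call and the current-skill assignment are disconnected and never run.
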(event `self.ReceiveBeginPlay`
  (bind _returnvalue (`GameplayStatics.GetActorOfClass` "/Game/Blueprints/Actors/Battle/BP_EnergySpawner.BP_EnergySpawner_C"))
  (set `self.EnergySpawner` _returnvalue))

(event `StartBossTurn`
  (`self.SetActorTickEnabled` true)
  (set `self.UseSkillPeriod` 10.0))

(event `EndBossTurn`
  (`self.SetActorTickEnabled` false))

(event `self.ReceiveTick`
  (params (DeltaSeconds :type "Float (single-precision)"))
  (bind _bossskillspawndatamap (`BattleTableManagerSystem.BossSkillSpawnDataMap` (subsystem `BattleTableManagerSystem`)))
  (bind _output_get (set `self.UseSkillPeriod` (+ DeltaSeconds (`self.UseSkillPeriod`))))
  (if (> _output_get 5.0)
    (set `self.UseSkillPeriod` 0.0)
    (bind _keys (`BlueprintMapLibrary.Map_Keys` _bossskillspawndatamap))
    (bind _value (`BlueprintMapLibrary.Map_Find` _bossskillspawndatamap (`KismetArrayLibrary.Array_Random` _keys)))
    (bind `_as액터` (castclass `Actor` (break `BossSkillSpawnData` _value)))
    (bind _returnvalue (`|SpawnActorFromClass` `_as액터` (`KismetArrayLibrary.Array_Random` (`.SkillTransform` (break `BossSkillSpawnData` _value))) "Undefined" "OverrideRootScale" null null))))

(fn `UserConstructionScript`)