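; Rose Queen boss actor that periodically attacks with spawned skill actors during battle.
; BossStarts enables Tick, which accumulates time and fires whenever the period exceeds five seconds.
; Each cycle spawns a random BossBattleSystem skill using BattleTableManagerSystem's class and transform data, then triggers EnergySpawner.
; Class and transform come from separate random skill lookups, so they can belong to different skills.
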(event `BossStarts`
  (`self.SetActorTickEnabled` true))

(event `self.ReceiveTick`
  (params (DeltaSeconds :type "Float (single-precision)"))
  (bind _value (`BlueprintMapLibrary.Map_Find` (`BattleTableManagerSystem.BossSkillSpawnDataMap` (subsystem `BattleTableManagerSystem`)) (`KismetArrayLibrary.Array_Random` (`BossBattleSystemComponent.BossSkillList` (`self.BossBattleSystem`)))))
  (bind _output_get (set `self.UseSkillPeriod` (+ DeltaSeconds (`self.UseSkillPeriod`))))
  (if (> _output_get 5.0)
    (set `self.UseSkillPeriod` 0.0)
    (bind `_as액터` (castclass `Actor` (break `BossSkillSpawnData` _value)))
    (`|SpawnActorFromClass` `_as액터` (`KismetArrayLibrary.Array_Random` (`.SkillTransform` (break `BossSkillSpawnData` _value))) "Undefined" "OverrideRootScale" null null)
    (`/Game/Blueprints/Actors/Battle/BP_EnergySpawner.Spawn Energy` (`self.EnergySpawner`))))

(fn `UserConstructionScript`)