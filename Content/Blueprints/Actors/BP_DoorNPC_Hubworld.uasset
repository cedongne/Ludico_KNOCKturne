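; BP_DoorNPC_Hubworld is the cabin door in the hub world, showing an "enter" interaction popup.
; BeginPlay sets the house door mesh and fills the popup widget's name and prompt with Korean text.
; SetCanInteraction and SetCannotInteraction toggle the interaction flags and popup visibility.
; The E key and Tick checks do nothing, and the hover outline and sound-then-load of LV_DreamWorld are disconnected.
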(event `BP Initialization 이벤트`
  ;[1 1 1] Init setting NPC
  (set `self.Mesh` (`self.HERBWORLDmodelling_house_door`)))

(event `Key|E`
  (params (Key :type "Key Structure"))
  (:`Pressed`
    (if (`SceneComponent.bHiddenInGame` (`self.Widget`))
      _)))

(event `self.ReceiveBeginPlay`
  ;[1 1 1] Set widget text block to its NPC name
  (`self.BP Initialization 이벤트`)
  (bind _asbp_interaction_popup (cast `/Game/Blueprints/UMG/BP_InteractionPopup` (`WidgetComponent.GetUserWidgetObject` (`self.Widget`))))
  (bind _output_get (set `self.InteractionUI` _asbp_interaction_popup))
  (`/Game/Blueprints/UMG/BP_InteractionPopup.Set NPC Interaction text` _output_get "오두막" "입장하기"))

(event `self.ReceiveTick`
  (params (DeltaSeconds :type "Float (single-precision)"))
  (if (`/Game/Blueprints/UMG/BP_InteractionPopup.isInteractionPossible` (`self.InteractionUI`))
    _))

(event `self.SetCanInteraction`
  ;[1 1 1] Check overlap to interaction capsule of Peppy : Show and hide interaction UI
  (set `NPCComponent.CanInteraction` true (`self.NPC`))
  (`SceneComponent.SetHiddenInGame` (`self.Widget`) false false)
  (set `/Game/Blueprints/UMG/BP_InteractionPopup.isInteractionPossible` true (`self.InteractionUI`)))

(event `self.SetCannotInteraction`
  ;[1 1 1] Check overlap to interaction capsule of Peppy : Show and hide interaction UI
  (set `NPCComponent.CanInteraction` false (`self.NPC`))
  (`SceneComponent.SetHiddenInGame` (`self.Widget`) true false)
  (set `/Game/Blueprints/UMG/BP_InteractionPopup.isInteractionPossible` false (`self.InteractionUI`)))

(fn `UserConstructionScript`)