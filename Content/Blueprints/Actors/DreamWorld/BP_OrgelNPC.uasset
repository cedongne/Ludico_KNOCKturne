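; BP_OrgelNPC is a Dream World NPC that shows an interaction popup and has an event to open the battle level.
; BeginPlay runs mesh setup and caches the widget component's BP_InteractionPopup.
; SetCanInteraction and SetCannotInteraction toggle the interaction flag and widget visibility.
; Hover outline logic and the button's click binding are disconnected, so this graph never hooks up the sound-and-level-load event.
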(event `BP Initialization 이벤트`
  ;[1 1 1] Init setting NPC
  (set `self.Mesh` (`self.herbworld_rabbitnpc`)))

(event `self.ReceiveBeginPlay`
  ;[1 1 1] Set widget text block to its NPC name
  (`self.BP Initialization 이벤트`)
  (bind _asbp_interaction_popup (cast `/Game/Blueprints/UMG/BP_InteractionPopup` (`WidgetComponent.GetUserWidgetObject` (`self.Widget`))))
  (set `self.InteractionUI` _asbp_interaction_popup))

(event `Interaction Button Click 이벤트`
  (`GameplayStatics.SpawnSoundAtLocation` null (0.0 0.0 0.0) (struct) 1.0 1.0 0.0 null null)
  (`GameplayStatics.OpenLevelBySoftObjectPtr` "/Game/Levels/LV_Battle.LV_Battle"))

(event `self.SetCanInteraction`
  ;[1 1 1] Check overlap to interaction capsule of Peppy : Show and hide interaction UI
  (set `NPCComponent.CanInteraction` true (`self.NPC`))
  (`SceneComponent.SetHiddenInGame` (`self.Widget`) false false))

(event `self.SetCannotInteraction`
  ;[1 1 1] Check overlap to interaction capsule of Peppy : Show and hide interaction UI
  (set `NPCComponent.CanInteraction` false (`self.NPC`))
  (`SceneComponent.SetHiddenInGame` (`self.Widget`) true false))

(fn `UserConstructionScript`)