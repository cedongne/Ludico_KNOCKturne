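; BP_Peppy is the player actor, handling NPC interaction and mouse-wheel camera zoom on its spring arm.
; Overlaps on its Interaction component toggle interactability on NPC-tagged actors.
; The interaction event blocks movement and sets a side-on camera target at the pair's midpoint, restoring the camera after a delay.
; Tick lerps the camera there with decelerating alpha steps while turning both actors toward each other.
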(event `self.Interaction.OnComponentBeginOverlap`
  (params (OverlappedComponent :type "PrimitiveComponent Object Reference") (OtherActor :type "Actor Object Reference") (OtherComp :type "PrimitiveComponent Object Reference") (OtherBodyIndex :type Integer) (bFromSweep :type Boolean) (SweepResult :type "HitResult Structure (by ref)"))
  ;[1 1 1] Check overlap to interaction capsule : Call SetCanInteraction event of overlapped interactionable actor
  (if (`self.ActorHasTag` OtherActor "NPC")
    (bind _asnpc (cast `NPC` OtherActor))
    (bind _output_get (set `self.OverlappedNPC` _asnpc))
    (`NPC.SetCanInteraction` _output_get)))

(event `self.Interaction.OnComponentEndOverlap`
  (params (OverlappedComponent :type "PrimitiveComponent Object Reference") (OtherActor :type "Actor Object Reference") (OtherComp :type "PrimitiveComponent Object Reference") (OtherBodyIndex :type Integer))
  ;[1 1 1] Check overlap to interaction capsule : Call SetCanInteraction event of overlapped interactionable actor
  (if (`self.ActorHasTag` OtherActor "NPC")
    (bind _asnpc (cast `NPC` OtherActor))
    (`NPC.SetCannotInteraction` _asnpc)))

(event `Interaction Camera Move 이벤트`
  (params (NPC :type "Pawn Object Reference"))
  (bind _returnvalue (`self.K2_GetActorLocation`))
  (bind _returnvalue_2 (`self.K2_GetActorLocation` NPC))
  (bind (_returnvalue_roll _returnvalue_pitch) (`KismetMathLibrary.BreakRotator` (`self.K2_GetActorRotation` NPC)))
  (bind (_returnvalue_roll_2 _returnvalue_pitch_2) (`KismetMathLibrary.BreakRotator` (`self.K2_GetActorRotation`)))
  (bind _overlappednpc (`self.OverlappedNPC`))
  (bind _camera (`self.Camera`))
  (bind _interactionviewpoint (`self.InteractionViewPoint`))
  (bind (_returnvalue_roll_3 _returnvalue_pitch_3 _returnvalue_yaw) (`KismetMathLibrary.BreakRotator` (`KismetMathLibrary.FindLookAtRotation` (`self.K2_GetActorLocation` NPC) _interactionviewpoint)))
  (bind (_returnvalue_roll_4 _returnvalue_pitch_4 _returnvalue_yaw_2) (`KismetMathLibrary.BreakRotator` (`KismetMathLibrary.FindLookAtRotation` (`self.K2_GetActorLocation`) _interactionviewpoint)))
  ;[1 1 1] Original interaction camera rotation
  (set `self.PrevCameraTransform` (`KismetMathLibrary.MakeTransform` (`SceneComponent.K2_GetComponentLocation` _camera) (`SceneComponent.K2_GetComponentRotation` _camera)))
  (bind _output_get (set `self.InteractionCameraLength` 400.0))
  (set `self.PrevPeppyLocation` _returnvalue_2)
  (bind _output_get_2 (set `self.InteractionViewPoint` (/ (+ _returnvalue _returnvalue_2) 2)))
  (if (>= (`KismetMathLibrary.DotProduct2D` (`KismetMathLibrary.Conv_VectorToVector2D` (- _returnvalue _returnvalue_2)) (`KismetMathLibrary.Conv_VectorToVector2D` (`SceneComponent.GetRightVector` _camera))) 0.0)
    (set `self.CameraAngle` (struct :`Yaw` -90.0))
    (else
      (set `self.CameraAngle` (struct :`Yaw` 90.0))))
  (bind _output_get_3 (set `self.InteractionCameraLocation` (* _output_get (`KismetMathLibrary.GreaterGreater_VectorRotator` (`KismetMathLibrary.GetDirectionUnitVector` _output_get_2 _returnvalue_2) (`self.CameraAngle`)))))
  (bind _output_get_4 (set `self.InteractionCameraLocation` (`KismetMathLibrary.MakeVector` (.x _output_get_3) (.y _output_get_3) 150.0)))
  (set `self.PrevPeppyRotation` (`KismetMathLibrary.MakeRotator` _returnvalue_roll_2 _returnvalue_pitch_2 _returnvalue_yaw_2))
  (set `self.PrevNPCRotation` (`KismetMathLibrary.MakeRotator` _returnvalue_roll _returnvalue_pitch _returnvalue_yaw))
  ;;[1 1 1] Init for interaction camera
  (set `self.InteractionCameraLocation` (+ _output_get_4 (`self.InteractionViewPoint`)))
  (set `self.CameraMoveSpeed` 0.03)
  (set `self.alpha` 0.0)
  (set `self.CanMove` false)
  (set `self.OnInteraction` true)
  (`NPC.SetCannotInteraction` _overlappednpc)
  (`KismetSystemLibrary.Delay` 3.0)
  ;;[1 1 1] Return camera transform
  (`SceneComponent.K2_SetWorldTransform` (`self.Camera`) (`self.PrevCameraTransform`) false false)
  (set `self.OnInteraction` false)
  (set `self.CanMove` true)
  (`NPC.SetCanInteraction` _overlappednpc))

(event `self.ReceiveTick`
  (params (DeltaSeconds :type "Float (single-precision)"))
  (bind _alpha (`self.alpha`))
  (bind _overlappednpc (`self.OverlappedNPC`))
  (bind _camera (`self.Camera`))
  (bind _prevcameratransform_location (`KismetMathLibrary.BreakTransform` (`self.PrevCameraTransform`)))
  (bind _alpha_2 (`self.alpha`))
  (bind _cameramovespeed (`self.CameraMoveSpeed`))
  (bind _returnvalue (`KismetMathLibrary.VLerp` _prevcameratransform_location (`self.InteractionCameraLocation`) (`self.alpha`)))
  (bind _returnvalue_2 (- _cameramovespeed 0.0003))
  ;[1 1 1] Original interaction camera rotation
  (if (`self.OnInteraction`)
    (`SceneComponent.K2_SetWorldLocation` _camera _returnvalue false false)
    (`SceneComponent.K2_SetWorldRotation` _camera (`KismetMathLibrary.FindLookAtRotation` _returnvalue (`KismetMathLibrary.VLerp` (`self.PrevPeppyLocation`) (`self.InteractionViewPoint`) (`self.alpha`))) false false)
    (`self.K2_SetActorRotation` (`KismetMathLibrary.RLerp` (`self.K2_GetActorRotation`) (`self.PrevPeppyRotation`) _alpha_2 true))
    (`self.K2_SetActorRotation` _overlappednpc (`KismetMathLibrary.RLerp` (`self.K2_GetActorRotation` _overlappednpc) (`self.PrevNPCRotation`) _alpha_2 true) false)
    (if (< _alpha 1.0)
      (set `self.alpha` (+ _alpha _cameramovespeed))
      (if (> _returnvalue_2 0.0)
        (set `self.CameraMoveSpeed` _returnvalue_2))
      (else
        (set `self.OnInteraction` false)))))

(event `Key|MouseScrollDown`
  (params (Key :type "Key Structure"))
  ;[1 1 1] Mouse wheel Zoom In and Zoom Out
  (:`Pressed`
    (set `SpringArmComponent.TargetArmLength` (`KismetMathLibrary.FClamp` (+ (`SpringArmComponent.TargetArmLength` (`self.SpringArm`)) 30.0) 200.0 800.0) (`self.SpringArm`))))

(event `Key|MouseScrollUp`
  (params (Key :type "Key Structure"))
  ;[1 1 1] Mouse wheel Zoom In and Zoom Out
  (:`Pressed`
    (set `SpringArmComponent.TargetArmLength` (`KismetMathLibrary.FClamp` (- (`SpringArmComponent.TargetArmLength` (`self.SpringArm`)) 30.0) 200.0 800.0) (`self.SpringArm`))))

(fn `UserConstructionScript`)