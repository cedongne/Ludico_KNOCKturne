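; BP_PS_ExhaustiveAdvice is a Peppy skill Blueprint that trades Peppy's positive buffs for damage.
; At effect sequence 1, CustomSkillOperation counts the per-second and per-turn positive buffs, then removes that many through RemoveRandomPositiveBuff.
; It deals count times the skill's ValueN to PeppyActor's own StatComponent, although the inline comment names the boss as target.
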(event `self.ReceiveBeginPlay`
  (`parent.ReceiveBeginPlay`))

(event `self.CustomSkillOperation`
  (params (EffectSequence :type Integer) (TargetActor :type "Actor Object Reference") (SkillData :type "CurEffectIndexSkillData Structure") (SkillActor :type "Actor Object Reference"))
  (bind _peppyactor (`ActorManagerSystem.PeppyActor` (subsystem `ActorManagerSystem`)))
  (bind _buffcomponent (`Peppy.BuffComponent` _peppyactor))
  ;[1 1 1] Effect 2. 페피가 가진 긍정적 버프들을 모두 제거하고, 보스에게 ‘제거된 버프의 개수*valueN’만큼의 데미지를 가합니다.
  (`KismetSystemLibrary.PrintString` "custom")
  (if (== EffectSequence 1)
    (bind _output_get (set `self.Positive Buffs Num` (+ (`BlueprintMapLibrary.Map_Length` (`BuffComponent.HasPositiveBuffs_PerSecond` _buffcomponent)) (`BlueprintMapLibrary.Map_Length` (`BuffComponent.HasPositiveBuffs_PerTurn` _buffcomponent)))))
    (`BuffComponent.RemoveRandomPositiveBuff` _buffcomponent _output_get)
    (`PeppyStatComponent.GetDamaged` (`Peppy.StatComponent` _peppyactor) (* (`self.Positive Buffs Num`) (`.Value_N` (break `CurEffectIndexSkillData` SkillData))))))

(fn `UserConstructionScript`
  (`parent.UserConstructionScript`))