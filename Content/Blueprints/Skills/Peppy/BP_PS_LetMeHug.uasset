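; Peppy's LetMeHug skill Blueprint, which randomly applies one of two battle effects.
; On BeginPlay it sets the PeppySkill audio switch, since skills sharing the animation need different sounds, then rolls an 80/20 choice of effect sequence.
; CustomSkillOperation acts only on the chosen sequence, swapping that outcome's skill index into the skill data and running it on the target through BattleTableManagerSystem.
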(event `self.ReceiveBeginPlay`
  (`AkGameplayStatics.SetSwitch` null null "PeppySkill" "EfficientEmpathy") ; 같은 애니메이션 사용을 하는 스킬들이 있어 사운드의 트리거를 각기 다르게 하기 위한 스위치 컴포넌트 입니다.
  (`parent.ReceiveBeginPlay`)
  (if (<= (`KismetMathLibrary.RandomFloat`) 0.8)
    (set `self.CanUseEffectSequence` 0)
    (else
      (set `self.CanUseEffectSequence` 1))))

(event `self.CustomSkillOperation`
  (params (EffectSequence :type Integer) (TargetActor :type "Actor Object Reference") (SkillData :type "CurEffectIndexSkillData Structure") (SkillActor :type "Actor Object Reference"))
  (if (== EffectSequence (`self.CanUseEffectSequence`))
    (if (== (`self.CanUseEffectSequence`) 0)
      (bind _structout (setmembers `CurEffectIndexSkillData` :`StructRef` SkillData :`SkillIndex` 16))
      (`BattleTableManagerSystem.OperateSkillByIndex` (subsystem `BattleTableManagerSystem`) 0 TargetActor _structout null)
      (else
        (bind _structout_2 (setmembers `CurEffectIndexSkillData` :`StructRef` SkillData :`SkillIndex` 34))
        (`BattleTableManagerSystem.OperateSkillByIndex` (subsystem `BattleTableManagerSystem`) 0 TargetActor _structout_2 null)))))

(fn `UserConstructionScript`
  (`parent.UserConstructionScript`))