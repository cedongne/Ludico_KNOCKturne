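; BP_PS_AmbiguousEmotion is a Peppy skill effect actor that shows an ambiguous emotion as three animated question marks.
; On BeginPlay it calls the parent and posts the Wwise Emotion event on the game mode actor.
; SpawnCustomEffect turns the Pivot toward Peppy's camera once per call, then plays each question mark widget component's own animation.
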(event `self.ReceiveBeginPlay`
  (`parent.ReceiveBeginPlay`)
  (`AkGameplayStatics.PostEvent` "/Game/Assets/Sounds/Wwise/Peppy/Emotion.Emotion" (`GameplayStatics.GetGameMode`)))

(fn `SpawnCustomEffect`
  (bind _aspeppy (cast `Peppy` (`GameplayStatics.GetPlayerCharacter` 0)))
  (`SceneComponent.K2_SetWorldRotation` (`self.Pivot`) (`KismetMathLibrary.FindLookAtRotation` (`SceneComponent.K2_GetComponentLocation` (`self.DefaultSceneRoot`)) (`SceneComponent.K2_GetComponentLocation` (`Peppy.Camera` _aspeppy))) false false)
  (bind _asbp_question_mark_1 (cast `/Game/Blueprints/UMG/BP_QuestionMark1` (`WidgetComponent.GetWidget` (`self.QuestionMark1`))))
  (`UserWidget.PlayAnimation` _asbp_question_mark_1 (`/Game/Blueprints/UMG/BP_QuestionMark1.QuestionMark1_Anim` _asbp_question_mark_1) 0.0 1 "Forward" 1.0 false)
  (bind _asbp_question_mark_2 (cast `/Game/Blueprints/UMG/BP_QuestionMark2` (`WidgetComponent.GetWidget` (`self.QuestionMark2`))))
  (`UserWidget.PlayAnimation` _asbp_question_mark_2 (`/Game/Blueprints/UMG/BP_QuestionMark2.QuestionMark2_Anim` _asbp_question_mark_2) 0.0 1 "Forward" 1.0 false)
  (bind _asbp_question_mark_3 (cast `/Game/Blueprints/UMG/BP_QuestionMark3` (`WidgetComponent.GetWidget` (`self.QuestionMark3`))))
  (`UserWidget.PlayAnimation` _asbp_question_mark_3 (`/Game/Blueprints/UMG/BP_QuestionMark3.QuestionMark3_Anim` _asbp_question_mark_3) 0.0 1 "Forward" 1.0 false))

(fn `UserConstructionScript`)