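; Peppy skill Charming Voice, which reduces the boss's EP by an amount that depends on Peppy's distance from the boss.
; It reads its row from the Peppy skill table, keyed by the Blueprint's own class name.
; Three distance bands, measured in PeppyMeter units, each select a table value to subtract through the boss's stat component.
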(event `self.ReceiveBeginPlay`
  (`parent.ReceiveBeginPlay`))

(event `self.CustomSkillOperation`
  (params (EffectSequence :type Integer) (TargetActor :type "Actor Object Reference") (SkillData :type "CurEffectIndexSkillData Structure") (SkillActor :type "Actor Object Reference"))
  (bind _returnvalue (* (`self.PeppyMeter`) 6))
  (bind _returnvalue_2 (* (`self.PeppyMeter`) 3))
  (bind _returnvalue_3 (`KismetMathLibrary.Vector_Distance` (`self.BossLocation`) (`self.K2_GetActorLocation` (`ActorManagerSystem.PeppyActor` (subsystem `ActorManagerSystem`)))))
  (bind _returnvalue_4 (`self.GetCurrentBlueprintClassName`))
  (bind _returnvalue_5 (`|GetDataTableRow` (`BattleTableManagerSystem.PeppySkillTable` (subsystem `BattleTableManagerSystem`)) _returnvalue_4)
    (:`then`
      (if (<= _returnvalue_3 _returnvalue_2)
        (bind (_skillid _skillgroupcode _skillacquire _cost _skillstance _skillcoolturn _skilldamagedelay _skillindex_1 _probability_1 _skilltarget_1 _value_1_n _value_1_m _value_1_t _buffcode_1 _skillindex_2 _probability_2 _skilltarget_2 _value_2_n _value_2_m _value_2_t _buffcode_2 _skillindex_3 _probability_3 _skilltarget_3 _value_3_n) (break `PeppySkillData` _returnvalue_5))
        (set `self.ReturnValue` _value_1_n)
        (`BossStatComponent.TryUpdateCurStatData` (`Boss.StatComponent` (`ActorManagerSystem.BossActor` (subsystem `ActorManagerSystem`))) "EP" (- 0.0 (`self.ReturnValue`)) :!label _label)
        (elif (and (> _returnvalue_3 _returnvalue_2) (<= _returnvalue_3 _returnvalue))
          (set `self.ReturnValue` _value_2_n)
          (goto _label)
          (elif (> _returnvalue_3 _returnvalue)
            (set `self.ReturnValue` _value_3_n)
            (goto _label)))))
    (:`RowNotFound`
      (`KismetSystemLibrary.PrintString` "RowName is ivanlid!"))))

(fn `UserConstructionScript`
  (`parent.UserConstructionScript`))