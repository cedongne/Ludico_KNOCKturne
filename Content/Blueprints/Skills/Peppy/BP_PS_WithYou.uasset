(event `self.ReceiveBeginPlay`
  (`parent.ReceiveBeginPlay`)
  (`AkGameplayStatics.PostEvent` "/Game/Assets/Sounds/Wwise/Peppy/WithYou.WithYou" (`GameplayStatics.GetGameMode`)))

(event `self.CustomSkillOperation`
  (params (EffectSequence :type Integer) (SkillData :type "CurEffectIndexSkillData Structure"))
  (bind (_skillid _skillindex _probability _skilltarget _value_n _value_m) (break `CurEffectIndexSkillData` SkillData))
  (bind _curbossstat (`BattleTableManagerSystem.CurBossStat` (subsystem `BattleTableManagerSystem`)))
  (bind _curpeppystat (`BattleTableManagerSystem.CurPeppyStat` (subsystem `BattleTableManagerSystem`)))
  (bind _returnvalue (`KismetMathLibrary.FTrunc` (- (`.EP` (break `BossStatData` _curbossstat)) _value_n)))
  ;[1 1 1] Effect 1-1. Probability_1의 확률로 보스에게 Value1N의 데미지를 가합니다.
  (if (<= (`KismetMathLibrary.RandomFloat`) _probability)
    (setmembers `BossStatData` :`StructRef` _curbossstat :`EP` _returnvalue)
    ;[1 1 1] Effect 1-2. 만약 페피의 HP가 Value1M 이하라면, 페피의 HP를 Value1N 만큼 증가시킵니다.
    (if (<= _returnvalue _value_m)
      (setmembers `PeppyStatData` :`StructRef` _curpeppystat :`EP` (`KismetMathLibrary.FTrunc` (+ _value_n (`.EP` (break `PeppyStatData` _curpeppystat))))))))

(fn `UserConstructionScript`
  (`parent.UserConstructionScript`))