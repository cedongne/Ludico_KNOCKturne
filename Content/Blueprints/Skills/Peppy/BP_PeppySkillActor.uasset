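; Base actor for Peppy's skills that snaps to the player's BP_Peppy pawn on BeginPlay and plays the skill's animation montage from its "Start" section.
; Skill data loads lazily from PeppySkillTable, using the current Blueprint class name as the row key.
; The montage is resolved through the Asset Registry from a path built with the row's animation name.
; A delay matches the montage length, with nothing wired after it.
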(event `self.ReceiveBeginPlay`
  (bind _asbp_peppy (cast `/Game/Blueprints/Actors/BP_Peppy` (`GameplayStatics.GetPlayerPawn` 0)))
  (`self.K2_SetActorTransform` self (`self.GetTransform` _asbp_peppy) false false)
  (`|ExecutionSequence`
    (:`then_0`
      (bind _newparam (`self.GetAnimMontageAsset`))
      (bind _returnvalue (`Character.PlayAnimMontage` _asbp_peppy _newparam 1.0 "Start"))
      (`KismetSystemLibrary.Delay` _returnvalue))))

(fn `GetAnimMontageAsset`
  (returns (NewParam :type "AnimMontage Object Reference"))
  (bind (_skillid _skillgroupcode _skillacquire _cost _skillstance _skillcoolturn _skilldamagedelay _skillindex_1 _probability_1 _skilltarget_1 _value_1_n _value_1_m _value_1_t _buffcode_1 _skillindex_2 _probability_2 _skilltarget_2 _value_2_n _value_2_m _value_2_t _buffcode_2 _skillindex_3 _probability_3 _skilltarget_3 _value_3_n _value_3_m _value_3_t _buffcode_3 _skillanimation) (break `PeppySkillData` (`self.SkillData`)))
  (bind _returnvalue (`KismetStringLibrary.Concat_StrStr` "/Game/Assets/Art_3D/Animation/Peppy_animation/" _skillanimation "." _skillanimation))
  (if (not (`self.IsSkillDataInitialized`))
    (`self.InitSkillData`))
  (bind _returnvalue_2 (`AssetRegistry.GetAssetByObjectPath` (`AssetRegistryHelpers.GetAssetRegistry`) (`KismetStringLibrary.Conv_StringToName` _returnvalue) false))
  (bind `_as애님_몽타주` (cast `AnimMontage` (`AssetRegistryHelpers.GetAsset` _returnvalue_2))
    (:`then`
      (return `_as애님_몽타주`))
    (:`CastFailed`
      (`KismetSystemLibrary.PrintString` (`KismetStringLibrary.Concat_StrStr` "[BP_PeppySkillData] AnimMontage assets is not found. " _returnvalue)))))

(fn `InitSkillData`
  (bind _returnvalue (`self.GetCurrentBlueprintClassName`))
  (bind _returnvalue_2 (`|GetDataTableRow` (`BattleTableManagerSystem.PeppySkillTable` (subsystem `BattleTableManagerSystem`)) _returnvalue)
    (:`then`
      (set `self.SkillData` _returnvalue_2)
      (set `self.IsSkillDataInitialized` true))
    (:`RowNotFound`
      (`KismetSystemLibrary.PrintString` (`KismetStringLibrary.Concat_StrStr` "[BP_PeppySkillActor] " (`KismetStringLibrary.Conv_NameToString` _returnvalue) " can't find.")))))

(fn `UserConstructionScript`)