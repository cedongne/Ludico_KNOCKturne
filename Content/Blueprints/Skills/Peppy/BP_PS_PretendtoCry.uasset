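; Peppy's "Pretend to Cry" battle skill, a probabilistic skill with two possible outcomes.
; On BeginPlay it posts an Ak audio event on the game mode and marks its usage type as probabilistic before running the parent logic.
; Its custom operation reads the probabilistic sequence from the battle table manager, rewrites the skill data to one of two skill indices, and has that manager execute it on the target.
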(event `self.ReceiveBeginPlay`
  (`AkGameplayStatics.PostEvent` "/Game/Assets/Sounds/Wwise/DoorHover.DoorHover" (`GameplayStatics.GetGameMode`))
  (set `self.Skill Using Type` "Probabilistic")
  (`parent.ReceiveBeginPlay`))

(event `self.CustomSkillOperation`
  (params (EffectSequence :type Integer) (TargetActor :type "Actor Object Reference") (SkillData :type "CurEffectIndexSkillData Structure") (SkillActor :type "Actor Object Reference"))
  (if (== (`BattleTableManagerSystem.PeppySkillProbabilisticSequence` (subsystem `BattleTableManagerSystem`)) 0)
    (bind _structout (setmembers `CurEffectIndexSkillData` :`StructRef` SkillData :`SkillIndex` 32))
    (`BattleTableManagerSystem.OperateSkillByIndex` (subsystem `BattleTableManagerSystem`) 0 TargetActor _structout null)
    (else
      (bind _structout_2 (setmembers `CurEffectIndexSkillData` :`StructRef` SkillData :`SkillIndex` 52))
      (`BattleTableManagerSystem.OperateSkillByIndex` (subsystem `BattleTableManagerSystem`) 0 TargetActor _structout_2 null))))

(fn `UserConstructionScript`
  (`parent.UserConstructionScript`))