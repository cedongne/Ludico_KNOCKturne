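; Starlight skill for Peppy that gives its target a Mood buff through the target's BuffComponent.
; A false CanGetMoodBuff flag blocks the buff for that use, and the flag resets to true afterward.
; Each spawn increments a BattleManager use counter; on reaching the skill table's threshold, the skill's cost is updated from that table and the counter resets.
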(event `self.ReceiveBeginPlay`
  (`/Engine/EditorBlueprintResources/StandardMacros.IncrementInt` (`BattleManagerSystem.UseStarlightNum` (subsystem `BattleManagerSystem`))
    (:`  `
      (`parent.ReceiveBeginPlay`))))

(event `self.CustomSkillOperation`
  (params (EffectSequence :type Integer) (TargetActor :type "Actor Object Reference") (SkillData :type "CurEffectIndexSkillData Structure") (SkillActor :type "Actor Object Reference"))
  (bind _returnvalue (`self.GetComponentByClass` TargetActor "/Script/KNOCKturne.BuffComponent"))
  (if (`BuffComponent.CanGetMoodBuff` _returnvalue)
    (`BuffComponent.AcquireBuff` _returnvalue "Mood" SkillData))
  (set `BuffComponent.CanGetMoodBuff` true _returnvalue)
  (`self.Increase Skill Cost`))

(fn `Increase Skill Cost`
  (bind _returnvalue (`self.GetCurrentBlueprintClassName`))
  (bind _returnvalue_2 (`|GetDataTableRow` (`BattleTableManagerSystem.PeppySkillTable` (subsystem `BattleTableManagerSystem`)) _returnvalue)
    (:`then`
      (bind (_skillid _skillgroupcode _skillacquire _cost _skillstance _skillcoolturn _skilldamagedelay _skillindex_1 _probability_1 _skilltarget_1 _value_1_n _value_1_m _value_1_t _buffcode_1 _skillindex_2 _probability_2 _skilltarget_2 _value_2_n _value_2_m _value_2_t _buffcode_2 _skillindex_3 _probability_3 _skilltarget_3 _value_3_n _value_3_m) (break `PeppySkillData` _returnvalue_2))
      (if (== (`BattleManagerSystem.UseStarlightNum` (subsystem `BattleManagerSystem`)) _value_3_n)
        (`BattleTableManagerSystem.TryUpdateCurSkillDataCost` (subsystem `BattleTableManagerSystem`) (`KismetSystemLibrary.GetClassDisplayName` (`GameplayStatics.GetObjectClass` self)) _value_3_m)
        (set `BattleManagerSystem.UseStarlightNum` 0 (subsystem `BattleManagerSystem`))
        (`KismetSystemLibrary.PrintString` (`KismetStringLibrary.Conv_IntToString` _cost))))))

(fn `UserConstructionScript`
  (`parent.UserConstructionScript`))