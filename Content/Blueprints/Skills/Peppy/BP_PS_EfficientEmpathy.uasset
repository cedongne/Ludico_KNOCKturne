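; Peppy skill Blueprint for Efficient Empathy, which restores Peppy's EP in battle when the boss's EP meets a condition.
; Its CustomSkillOperation event handles only the second effect (sequence index 1), checking whether the boss's current EP ends in zero.
; On a match, it adds the skill's ValueN to Peppy's current EP in the battle table manager's stat data, truncating the result.
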(event `self.ReceiveBeginPlay`
  (`parent.ReceiveBeginPlay`))

(event `self.CustomSkillOperation`
  (params (EffectSequence :type Integer) (SkillData :type "CurEffectIndexSkillData Structure"))
  (bind _returnvalue (subsystem `BattleTableManagerSystem`))
  (bind (_curbossstat_bossmindelay _curbossstat_bossmaxdelay _curbossstat_bossstancecode _curbossstat_bossinitstance _curbossstat_bossenergydrop _curbossstat_ep) (break `BossStatData` (`BattleTableManagerSystem.CurBossStat` _returnvalue)))
  (bind _curpeppystat (`BattleTableManagerSystem.CurPeppyStat` _returnvalue))
  ;[1 1 1] Effect 2. 보스 EP의 일의 단위가 0이라면, 페피의 EP를  Value1N만큼 회복시킵니다.
  (if (and (== EffectSequence 1) (== (mod _curbossstat_ep 10) 0))
    (setmembers `PeppyStatData` :`StructRef` _curpeppystat :`EP` (`KismetMathLibrary.FTrunc` (+ (`.EP` (break `PeppyStatData` _curpeppystat)) (`.Value_N` (break `CurEffectIndexSkillData` SkillData)))))))

(fn `UserConstructionScript`
  (`parent.UserConstructionScript`))