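; BP_SpecialSkillActor is a special skill actor that sets up the Niagara visual effect for a skill in battle.
; SpawnEffect assigns the resolved system to its Effect component, except when the battle manager's final special skill is Gatherenergy.
; The system is looked up by name through the Asset Registry, using a path built from SpecialSkillData's effect name under the SpecialSkillEffect folder, and a missing asset prints an error.
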(fn `GetNiagaraEffectAsset`
  (returns (`Niagara System Asset` :type "NiagaraSystem Object Reference"))
  (locals (`Effect Name` :type String))
  (bind _effect_name (`local.Effect Name`))
  (set `local.Effect Name` (`.SpecialSkillEffect` (break `SpecialSkillTable` (`self.SpecialSkillData`))))
  (bind _returnvalue (`AssetRegistry.GetAssetByObjectPath` (`AssetRegistryHelpers.GetAssetRegistry`) (`KismetStringLibrary.Conv_StringToName` (`KismetStringLibrary.Concat_StrStr` "/Game/Assets/Effects/SpecialSkillEffect/" _effect_name "." _effect_name)) false))
  (bind `_as나이아가라_시스템` (cast `NiagaraSystem` (`AssetRegistryHelpers.GetAsset` _returnvalue))
    (:`then`
      (return `_as나이아가라_시스템`))
    (:`CastFailed`
      (`KismetSystemLibrary.PrintString` (`KismetStringLibrary.Concat_StrStr` "[BP_SpecialSkillActor] NiagaraEffect asset is not found: " (`local.Effect Name`))))))

(fn `SpawnEffect`
  (if (`KismetStringLibrary.NotEqual_StrStr` (`BattleManagerSystem.FinalSpecialSkill` (subsystem `BattleManagerSystem`)) "Skill_Special_Gatherenergy")
    (bind _niagara_system_asset (`self.GetNiagaraEffectAsset`))
    (`/Engine/EditorBlueprintResources/StandardMacros.IsValid` _niagara_system_asset
      (:`Is Valid`
        (`NiagaraComponent.SetAsset` (`self.Effect`) _niagara_system_asset true)))))

(fn `UserConstructionScript`)