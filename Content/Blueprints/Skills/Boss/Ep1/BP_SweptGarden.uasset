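; Episode 1 boss skill actor for Swept Garden, an attack that sweeps a hit collision forward to damage Peppy.
; BeginPlay loads its BossSkillTable row and registers AttackRange as the current boss hit area.
; After a short delay it removes that area, unpauses the bone animation and Tick slides HitCollision along local X until the actor self-destructs.
; Overlaps hit Peppy if not already hit; an unused chained-spawn mechanism remains, marked discarded.
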(event `self.ReceiveBeginPlay`
  (bind _returnvalue (subsystem `BattleManagerSystem`))
  (bind _attackrange (`self.AttackRange`))
  ;[1 1 1] Initialization
  ;;[1 1 1] Value Type
  (set `self.CollisionMoveTime` 0.0)
  ;;[1 1 1] Reference Type
  (bind _returnvalue_2 (`|GetDataTableRow` (`BattleTableManagerSystem.BossSkillTable` (subsystem `BattleTableManagerSystem`)) "BP_SweptGarden_C")
    (:`then`
      (`self.SetSkillData` _returnvalue_2)
      (set `self.SkillHitArea` _attackrange)
      (bind _output_get (set `BattleManagerSystem.CurBossSkillHitArea` _attackrange _returnvalue))
      (`SceneComponent.SetHiddenInGame` _output_get (not (`BattleManagerSystem.VisibleBossSkillHitArea` _returnvalue)) false)
      (`KismetSystemLibrary.Delay` 1.0)
      (set `SkeletalMeshComponent.bPauseAnims` false (`self.Ani_SweptGarden_bone`))
      (`ActorComponent.K2_DestroyComponent` (`self.AttackRange`))
      (`KismetSystemLibrary.Delay` 1.5)
      (`self.K2_DestroyActor`))))

(event `self.HitCollision.OnComponentBeginOverlap`
  (params (OverlappedComponent :type "PrimitiveComponent Object Reference") (OtherActor :type "Actor Object Reference") (OtherComp :type "PrimitiveComponent Object Reference") (OtherBodyIndex :type Integer) (bFromSweep :type Boolean) (SweepResult :type "HitResult Structure (by ref)"))
  (if (== (`PrimitiveComponent.GetCollisionProfileName` OtherComp) "Peppy")
    (bind _asbp_peppy (cast `/Game/Blueprints/Actors/BP_Peppy` OtherActor))
    (if (`Peppy.IsHit` _asbp_peppy)
      _
      (elif (`self.IsInitialized`)
        (`self.HitPlayer`)
        (`/Game/Blueprints/Actors/BP_Peppy.Hit` _asbp_peppy)))))

(event `self.ReceiveTick`
  (params (DeltaSeconds :type "Float (single-precision)"))
  (bind _output_get (set `self.CollisionMoveTime` (+ DeltaSeconds (`self.CollisionMoveTime`))))
  (if (>= _output_get 1.0)
    (bind _returnvalue (`self.GetDeltaDurationMove` (0.0 0.0 0.0) (800.0 0.0 0.0) 1.5 DeltaSeconds))
    (`SceneComponent.K2_AddRelativeLocation` (`self.HitCollision`) _returnvalue false false)))

(fn `UserConstructionScript`)