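; BP_CleanUpIntruder1 is an Episode 1 boss skill actor that launches the CleanUp attack by spawning two BP_CleanUpIntruder1_Unit actors.
; On BeginPlay it posts the CleanUp Wwise event on the game mode, then rolls two distinct random indices out of three.
; Both units share one hardcoded location, with each index multiplying a 90-degree base rotation to give them different orientations.
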(event `self.ReceiveBeginPlay`
  (bind (_spawntransformbase_location _spawntransformbase_rotation) (`KismetMathLibrary.BreakTransform` (`self.SpawnTransformBase`)))
  (bind (_spawntransformbase_location_2 _spawntransformbase_rotation_2) (`KismetMathLibrary.BreakTransform` (`self.SpawnTransformBase`)))
  (`AkGameplayStatics.PostEvent` "/Game/Assets/Sounds/Wwise/Battle/CleanUp.CleanUp" (`GameplayStatics.GetGameMode`))
  (set `self.SpawnTransformBase` (`KismetMathLibrary.MakeTransform` (755.0 771.0 -86.0) (struct :`Yaw` 90.0)))
  (bind _output_get (set `self.FirstTransformIndex` (`KismetMathLibrary.RandomInteger` 3)))
  (bind _output_get_2 (set `self.SecondTransformIndex` (`KismetMathLibrary.RandomInteger` 3)))
  (while (== _output_get_2 _output_get)
    (set `self.SecondTransformIndex` (`KismetMathLibrary.RandomInteger` 3)))
  (`|SpawnActorFromClass` "/Game/Blueprints/Skills/Boss/Ep1/SkillActor/BP_CleanUpIntruder1_Unit.BP_CleanUpIntruder1_Unit_C" (`KismetMathLibrary.MakeTransform` _spawntransformbase_location (* _spawntransformbase_rotation (`self.FirstTransformIndex`))) "Undefined" "OverrideRootScale" null null)
  (`|SpawnActorFromClass` "/Game/Blueprints/Skills/Boss/Ep1/SkillActor/BP_CleanUpIntruder1_Unit.BP_CleanUpIntruder1_Unit_C" (`KismetMathLibrary.MakeTransform` _spawntransformbase_location_2 (* _spawntransformbase_rotation_2 (`self.SecondTransformIndex`))) "Undefined" "OverrideRootScale" null null))

(fn `UserConstructionScript`)