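; Boss skill actor for Episode 1's GoBackMoment flower, a timed challenge to collect every yellow petal.
; Tick follows the skill step: the flower rises during delay, polls for remaining yellow petal actors during cast, and damages the player once at destroy time.
; When no yellow petals remain, it turns yellow, ends the gray petals and itself, then spawns the next boss skill.
; Overlapping the flower makes the player temporarily immune to damage.
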(event `self.ReceiveBeginPlay`
  (`parent.ReceiveBeginPlay`))

(event `self.ReceiveTick`
  (params (DeltaSeconds :type "Float (single-precision)"))
  (bind _output_get (set `self.DeltaTime` DeltaSeconds))
  (`parent.ReceiveTick` _output_get)
  (bind _returnvalue (`self.GetSkillData`))
  (switch `ESkillActorLifeCycleStep` (`self.CurrentStep`)
    (:`DelayTime`
      (`self.LinearTransformInDuration` (0.0 0.0 280.0) (`.SkillDelayTime` (break `BossSkillData` _returnvalue))))
    (:`CastTime`
      (`self.Check If Collected All Yellow Petals`))
    (:`DestroyTime`
      (`/Engine/EditorBlueprintResources/StandardMacros.DoOnce` false
        (:`Completed`
          (`self.Not Gathered In Time`))))))

(event `End Cur Skill and Spawn New Boss Skill`
  (bind _outactors (`GameplayStatics.GetAllActorsOfClass` "/Game/Blueprints/Skills/Boss/Ep1/SkillActor/BP_GoBackMoment_GrayPetal.BP_GoBackMoment_GrayPetal_C"))
  (for _array_element _outactors
    (`self.EndCurBossSkill` _array_element))
  (`self.EndCurBossSkillAfterSec` 1.0)
  (`self.StopAndSpawnNewBossSkill`))

(event `self.ReceiveActorBeginOverlap`
  (params (OtherActor :type "Actor Object Reference"))
  (bind _returnvalue (`GameplayStatics.GetPlayerPawn` 0))
  (if (== OtherActor _returnvalue)
    (bind _aspeppy (cast `Peppy` _returnvalue))
    (set `PeppyStatComponent.CanBeDamaged` false (`Peppy.StatComponent` _aspeppy))))

(event `self.ReceiveActorEndOverlap`
  (params (OtherActor :type "Actor Object Reference"))
  (bind _returnvalue (`GameplayStatics.GetPlayerPawn` 0))
  (if (== OtherActor _returnvalue)
    (bind _aspeppy (cast `Peppy` _returnvalue))
    (set `PeppyStatComponent.CanBeDamaged` true (`Peppy.StatComponent` _aspeppy))))

(fn `Check If Collected All Yellow Petals`
  (bind _outactors (`GameplayStatics.GetAllActorsOfClass` "/Game/Blueprints/Skills/Boss/Ep1/SkillActor/BP_GoBackMoment_YellowPetal.BP_GoBackMoment_YellowPetal_C"))
  (if (== (`KismetArrayLibrary.Array_Length` _outactors) 0)
    (`StaticMeshComponent.SetStaticMesh` (`self.SkillMesh`) "/Game/Assets/Art_3D/Modelling/skill_modelling/Md_BossSkill_YellowFlower.Md_BossSkill_YellowFlower")
    (`self.End Cur Skill and Spawn New Boss Skill`)))

(fn `LinearTransformInDuration`
  (params (Movement :type "Vector Structure") (Duration :type "Float (double-precision)"))
  (`self.GetSkillData`)
  (`SceneComponent.K2_AddRelativeLocation` (`self.SkillMeshPivot`) (* Movement (/ (`self.DeltaTime`) Duration)) false false))

(fn `Not Gathered In Time`
  (bind _returnvalue (`self.GetSkillData`))
  (bind _asbp_peppy (cast `/Game/Blueprints/Actors/BP_Peppy` (`GameplayStatics.GetPlayerCharacter` 0)))
  (`PeppyStatComponent.GetDamaged` (`Peppy.StatComponent` _asbp_peppy) (`.Value_1_M` (break `BossSkillData` _returnvalue))))

(fn `UserConstructionScript`
  (`parent.UserConstructionScript`))