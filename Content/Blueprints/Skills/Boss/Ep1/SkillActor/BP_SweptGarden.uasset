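; Boss skill actor for Swept Garden in Ep1, with a hit collision that travels forward along local X.
; BeginPlay asks the parent skill logic to start the bone animation after the skill delay.
; Tick accumulates elapsed time and, during the cast window that follows the delay, offsets HitCollision by a per-frame step from a fixed distance and duration, without sweeping.
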(event `self.ReceiveBeginPlay`
  (`parent.ReceiveBeginPlay`)
  (set `self.CollisionMoveTime` 0.0)
  (`self.StartSkillAnimationAfterSkillDelayTime` (`self.Ani_SweptGarden_bone`)))

(event `self.ReceiveTick`
  (params (DeltaSeconds :type "Float (single-precision)"))
  (`parent.ReceiveTick` DeltaSeconds)
  (bind _output_get (set `self.CollisionMoveTime` (+ DeltaSeconds (`self.CollisionMoveTime`))))
  (bind _returnvalue (`self.GetSkillData`))
  (bind (_bossskillid _skillstance _skillcoolturn _sprayenergy _skilldelaytime _skillcasttime) (break `BossSkillData` _returnvalue))
  (if (`KismetMathLibrary.InRange_FloatFloat` _output_get _skilldelaytime (+ _skilldelaytime _skillcasttime))
    (bind _returnvalue_2 (`self.GetDeltaDurationMove` (0.0 0.0 0.0) (800.0 0.0 0.0) 2.0 DeltaSeconds))
    (`SceneComponent.K2_AddRelativeLocation` (`self.HitCollision`) _returnvalue_2 false false)))

(fn `UserConstructionScript`)