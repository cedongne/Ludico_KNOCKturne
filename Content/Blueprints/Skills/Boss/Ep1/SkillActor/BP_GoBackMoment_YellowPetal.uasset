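; Episode 1 boss skill actor for the yellow petal of the GoBackMoment skill, built on a parent that provides skill data and step state.
; During the Delay Time step, Tick raises the mesh pivot 100 units along relative Z, spread over the skill's delay time by scaling with delta time.
; On overlap with the Peppy player pawn, it destroys itself, switching the player's CanBeDamaged off just before and back on immediately after.
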(event `self.ReceiveBeginPlay`
  (`parent.ReceiveBeginPlay`))

(event `self.ReceiveTick`
  (params (DeltaSeconds :type "Float (single-precision)"))
  (bind _output_get (set `self.DeltaTime` DeltaSeconds))
  (`parent.ReceiveTick` _output_get)
  (bind _returnvalue (`self.GetSkillData`))
  (switch `ESkillActorLifeCycleStep` (`self.CurrentStep`)
    (:`DelayTime`
      (`self.LinearTransformInDuration` (0.0 0.0 100.0) (`.SkillDelayTime` (break `BossSkillData` _returnvalue))))))

(event `self.ReceiveActorBeginOverlap`
  (params (OtherActor :type "Actor Object Reference"))
  (bind _returnvalue (`GameplayStatics.GetPlayerPawn` 0))
  (if (== OtherActor _returnvalue)
    (bind _aspeppy (cast `Peppy` _returnvalue))
    (bind _statcomponent (`Peppy.StatComponent` _aspeppy))
    (set `PeppyStatComponent.CanBeDamaged` false _statcomponent)
    (`self.K2_DestroyActor`)
    (set `PeppyStatComponent.CanBeDamaged` true _statcomponent)))

(fn `LinearTransformInDuration`
  (params (Movement :type "Vector Structure") (Duration :type "Float (double-precision)"))
  (`self.GetSkillData`)
  (`SceneComponent.K2_AddRelativeLocation` (`self.SkillMeshPivot`) (* Movement (/ (`self.DeltaTime`) Duration)) false false))

(fn `UserConstructionScript`
  (`parent.UserConstructionScript`))