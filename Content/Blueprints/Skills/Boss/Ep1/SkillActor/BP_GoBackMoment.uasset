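; Boss episode 1 GoBackMoment skill actor that, on BeginPlay, plays its sound and spawns a central flower plus five petals, randomly split between yellow and gray.
; Petal transforms get random yaw and a point in a fixed box, re-rolled only while yellow, gray and flower proximity checks all report overlap.
; Each petal gets a random mesh from its color's set; the used-index list clears per call, so meshes can repeat.
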(event `self.ReceiveBeginPlay`
  (`AkGameplayStatics.PostEvent` "/Game/Assets/Sounds/Wwise/Play_Boss_GoBackMoment.Play_Boss_GoBackMoment" (`GameplayStatics.GetGameMode`))
  (`|SpawnActorFromClass` "/Game/Blueprints/Skills/Boss/Ep1/SkillActor/BP_GoBackMoment_Flower.BP_GoBackMoment_Flower_C" (`KismetMathLibrary.MakeTransform` (755.0 771.0 -86.0)) "Undefined" "OverrideRootScale" null null)
  (bind _output_get (set `self.Yellow Petal Num` (`KismetMathLibrary.RandomIntegerInRange` 2 4)))
  (set `self.Gray Petal Num` (- 5 _output_get))
  (`self.Spawn Boss Skill Actor` (`self.Yellow Petal Num`) "/Game/Blueprints/Skills/Boss/Ep1/SkillActor/BP_GoBackMoment_YellowPetal.BP_GoBackMoment_YellowPetal_C" (`self.Yellow Petal Transforms`))
  (`self.Spawn Boss Skill Actor` (`self.Gray Petal Num`) "/Game/Blueprints/Skills/Boss/Ep1/SkillActor/BP_GoBackMoment_GrayPetal.BP_GoBackMoment_GrayPetal_C" (`self.Gray Petal Transforms`)))

(fn `Check If Overlapping`
  (params (`Cur Skill` :type "Vector Structure") (`Actor Location` :type "Vector Structure") (Range :type Integer))
  (returns (Overlapping :type Boolean))
  (bind _returnvalue (`BattleUtilManager.InRangeLocation` (subsystem `BattleUtilManager`) `Cur Skill` (- `Actor Location` Range) (+ `Actor Location` Range)))
  (return _returnvalue))

(fn `Set Petal Static Mesh`
  (params (`BP_BossSkill Ref` :type "/Game/Blueprints/Skills/Boss/Ep1/SkillActor/BP_BossSkillActor Object Reference") (`Is Yellow Petal` :type Boolean))
  (locals (`Petal Static Meshs` :type "Array of StaticMesh Object Reference") (`Random Index` :type Integer))
  (bind _bp_bossskill_ref (`local.BP_BossSkill Ref`))
  (`KismetArrayLibrary.Array_Clear` (`self.Used Static Mesh Num`))
  (if `Is Yellow Petal`
    (set `local.Petal Static Meshs` (`self.Yellow Petal Static Meshs`))
    (else
      (set `local.Petal Static Meshs` (`self.Gray Petal Static Meshs`))))
  (set `local.Random Index` (`KismetMathLibrary.RandomInteger` 6) :!label _label)
  (if (`KismetArrayLibrary.Array_Contains` (`self.Used Static Mesh Num`) (`local.Random Index`))
    (goto _label)
    (else
      (`/Engine/EditorBlueprintResources/StandardMacros.IsValid` _bp_bossskill_ref
        (:`Is Valid`
          (`StaticMeshComponent.SetStaticMesh` (`BossSkillActor.SkillMesh` _bp_bossskill_ref) (`|GetArrayItem` (`local.Petal Static Meshs`) (`local.Random Index`)))
          (`KismetArrayLibrary.Array_Add` (`self.Used Static Mesh Num`) (`local.Random Index`)))))))

(fn `SetRandomSkillTransform`
  (returns (SkillTansform :type "Transform Structure"))
  (locals (Index :type Integer))
  (bind _output_get (set `self.IsOverlap` true))
  (while _output_get
    (bind _output_get_2 (set `self.CurrentIndexLocation` (`KismetMathLibrary.RandomPointInBoundingBox` (751.0 774.0 -87.0) (400.0 400.0 0.0))))
    (bind _returnvalue (`BattleUtilManager.IsOverlappedAnotherSkills` (subsystem `BattleUtilManager`) _output_get_2 (`self.Yellow Petal Transforms`) 300))
    (bind _returnvalue_2 (`BattleUtilManager.IsOverlappedAnotherSkills` (subsystem `BattleUtilManager`) (`self.CurrentIndexLocation`) (`self.Gray Petal Transforms`) 300))
    (bind _returnvalue_3 (`GameplayStatics.GetActorOfClass` "/Game/Blueprints/Skills/Boss/Ep1/SkillActor/BP_GoBackMoment_Flower.BP_GoBackMoment_Flower_C"))
    (bind _overlapping (`self.Check If Overlapping` (`self.CurrentIndexLocation`) (`self.K2_GetActorLocation` _returnvalue_3) 300))
    (set `self.IsOverlap` (and _returnvalue _returnvalue_2 _overlapping)))
  (return (`KismetMathLibrary.MakeTransform` (`self.CurrentIndexLocation`) (`KismetMathLibrary.MakeRotator` 0.0 0.0 (`KismetMathLibrary.RandomFloatInRange` 0.0 360.0)))))

(fn `Spawn Boss Skill Actor`
  (params (`Actor Num` :type Integer) (`Actor Class` :type "Actor Class Reference") (`Skill Transforms` :type "Array of Transform Structure"))
  (for _ (range `Actor Num`)
    (bind _skilltansform (`self.SetRandomSkillTransform`))
    (`KismetArrayLibrary.Array_Add` (`local.Skill Transforms`) _skilltansform))
  (for _array_element (`local.Skill Transforms`)
    (bind _returnvalue (`|SpawnActorFromClass` (`local.Actor Class`) _array_element "Undefined" "OverrideRootScale" null null))
    (bind _asbp_boss_skill_actor (cast `/Game/Blueprints/Skills/Boss/Ep1/SkillActor/BP_BossSkillActor` _returnvalue))
    (if (== (`GameplayStatics.GetObjectClass` _returnvalue) "/Game/Blueprints/Skills/Boss/Ep1/SkillActor/BP_GoBackMoment_YellowPetal.BP_GoBackMoment_YellowPetal_C")
      (`self.Set Petal Static Mesh` _asbp_boss_skill_actor true)
      (else
        (`self.Set Petal Static Mesh` _asbp_boss_skill_actor)))))

(fn `UserConstructionScript`)