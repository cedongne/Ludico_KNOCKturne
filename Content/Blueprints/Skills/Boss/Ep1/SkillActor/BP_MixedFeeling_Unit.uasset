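; Episode 1 boss skill actor for one Mixed Feeling unit, which damages Peppy through its custom skill operation.
; During Delay Time it tracks the player on one axis set by IsVertical, optionally showing its hit area, then hides that and raises the mesh.
; During Cast Time it slides in one of two random directions and destroys itself off-field.
; When no units remain, it calls for the next boss skill.
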(event `self.ReceiveBeginPlay`
  (`parent.ReceiveBeginPlay`))

(event `self.ReceiveTick`
  (params (DeltaSeconds :type "Float (single-precision)"))
  (bind _output_get (set `self.DeltaTime` DeltaSeconds))
  (`parent.ReceiveTick` _output_get)
  (bind _returnvalue (`self.GetSkillData`))
  (switch `ESkillActorLifeCycleStep` (`self.CurrentStep`)
    (:`DelayTime`
      (bind _output_get_2 (set `self.Thorny Vine Follow Time` (+ (`self.DeltaTime`) (`self.Thorny Vine Follow Time`))))
      (if (<= _output_get_2 1.0)
        (`self.SetAttackRangeForSkillVis`)
        (`self.Follow Player`)
        (else
          (`SceneComponent.SetVisibility` (`self.AttackRangeForSkill`) false false)
          ;[1 0.2917 0.2917] 모델링 변경 후 Movement 변경 필요
          (`self.LinearTransformInDuration` (0.0 0.0 30.0) 1.0))))
    (:`CastTime`
      (`self.Move Random Dir`)
      (`self.Check If Go Off Field`))))

(event `self.CustomSkillOperation`
  (params (EffectSequence :type Integer) (TargetActor :type "Actor Object Reference") (SkillData :type "CurEffectIndexSkillData Structure") (SkillActor :type "Actor Object Reference"))
  (bind _asbp_peppy (cast `/Game/Blueprints/Actors/BP_Peppy` (`GameplayStatics.GetPlayerCharacter` 0)))
  (`PeppyStatComponent.GetDamaged` (`Peppy.StatComponent` _asbp_peppy) (`.Value_N` (break `CurEffectIndexSkillData` SkillData))))

(fn `Check If Go Off Field`
  (locals (NewLocalVar_0 :type "Vector Structure"))
  (bind _returnvalue_x (`KismetMathLibrary.BreakVector` (`SceneComponent.K2_GetComponentLocation` (`self.SkillMesh`))))
  (bind (_returnvalue_x_2 _returnvalue_y) (`KismetMathLibrary.BreakVector` (`SceneComponent.K2_GetComponentLocation` (`self.SkillMesh`))))
  (if (`self.IsVertical`)
    (if (or (>= _returnvalue_y 1270.0) (<= _returnvalue_y 270.0))
      (`self.K2_DestroyActor` :!label _label)
      (bind _outactors (`GameplayStatics.GetAllActorsOfClass` "BP_MixedFeeling_Unit_C"))
      (if (== (`KismetArrayLibrary.Array_Length` _outactors) 0)
        (`self.StopAndSpawnNewBossSkill`)))
    (elif (or (>= _returnvalue_x 1250.0) (<= _returnvalue_x 250.0))
      (goto _label))))

(fn `Follow Player`
  (locals (Location :type "Vector Structure" :default (0.0 0.0 0.0)))
  (bind (_returnvalue_x _returnvalue_y _returnvalue_z) (`KismetMathLibrary.BreakVector` (`self.K2_GetActorLocation`)))
  (bind (_returnvalue_x_2 _returnvalue_y_2 _returnvalue_z_2) (`KismetMathLibrary.BreakVector` (`self.K2_GetActorLocation`)))
  (bind _returnvalue_x_3 (`KismetMathLibrary.BreakVector` (`self.K2_GetActorLocation` (`GameplayStatics.GetPlayerPawn` 0))))
  (bind (_returnvalue_x_4 _returnvalue_y_3) (`KismetMathLibrary.BreakVector` (`self.K2_GetActorLocation` (`GameplayStatics.GetPlayerPawn` 0))))
  (if (`self.IsVertical`)
    (set `local.Location` (`KismetMathLibrary.MakeVector` _returnvalue_x _returnvalue_y_3 _returnvalue_z))
    (else
      (set `local.Location` (`KismetMathLibrary.MakeVector` _returnvalue_x_3 _returnvalue_y_2 _returnvalue_z_2))))
  (`self.K2_SetActorLocation` (`local.Location`)))

(fn `Follow Player2`
  (locals (Location :type "Vector Structure" :default (0.0 0.0 0.0)))
  (bind (_returnvalue_x _returnvalue_y _returnvalue_z) (`KismetMathLibrary.BreakVector` (`self.K2_GetActorLocation`)))
  (bind (_returnvalue_x_2 _returnvalue_y_2 _returnvalue_z_2) (`KismetMathLibrary.BreakVector` (`self.K2_GetActorLocation`)))
  (bind _returnvalue_x_3 (`KismetMathLibrary.BreakVector` (`self.K2_GetActorLocation` (`GameplayStatics.GetPlayerPawn` 0))))
  (bind (_returnvalue_x_4 _returnvalue_y_3) (`KismetMathLibrary.BreakVector` (`self.K2_GetActorLocation` (`GameplayStatics.GetPlayerPawn` 0))))
  (if (`self.IsVertical`)
    (set `local.Location` (`KismetMathLibrary.MakeVector` _returnvalue_x _returnvalue_y_3 _returnvalue_z))
    (else
      (set `local.Location` (`KismetMathLibrary.MakeVector` _returnvalue_x_3 _returnvalue_y_2 _returnvalue_z_2))))
  (`self.K2_SetActorLocation` (`local.Location`)))

(fn `LinearTransformInDuration`
  (params (Movement :type "Vector Structure") (Duration :type "Float (double-precision)"))
  (`self.GetSkillData`)
  (`SceneComponent.K2_AddRelativeLocation` (`self.SkillMeshPivot`) (* Movement (/ (`self.DeltaTime`) Duration)) false false))

(fn `Move Random Dir`
  (locals (`Vertical Dir` :type "Array of Vector Structure") (`Horizontal Dir` :type "Array of Vector Structure") (`Random Movement` :type "Vector Structure"))
  (if (== (.x (`self.Random Direction`)) 0.0)
    (`self.Set Random Dir`)
    (else
      (`self.LinearTransformInDuration` (`self.Random Direction`) 1.0))))

(fn `Set Random Dir`
  (locals (`Random Dir` :type "Array of Vector Structure"))
  (set `self.Random Direction` (`|GetArrayItem` (`local.Random Dir`) (`KismetMathLibrary.RandomInteger` 2))))

(fn `SetAttackRangeForSkillVis`
  (bind _returnvalue (`GameplayStatics.GetActorOfClass` "/Game/Blueprints/Actors/Battle/BP_BattleFoothold.BP_BattleFoothold_C"))
  (`/Engine/EditorBlueprintResources/StandardMacros.IsValid` _returnvalue
    (:`Is Valid`
      (if (`BattleManagerSystem.VisibleBossSkillHitArea` (subsystem `BattleManagerSystem`))
        (`SceneComponent.SetVisibility` (`self.AttackRangeForSkill`) true false)
        (else
          (`SceneComponent.SetVisibility` (`self.AttackRangeForSkill`) false false))))))

(fn `UserConstructionScript`
  (`parent.UserConstructionScript`))