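; Boss skill actor for the Ep1 GoBackMoment GrayPetal attack, built on a parent skill actor that supplies step state and skill data.
; During the Delay Time step, Tick moves the mesh pivot upward at a frame-scaled rate spread over the skill's delay duration.
; The custom skill operation applies the skill's value as damage directly to the player's BP_Peppy stat component, with no overlap check here, then destroys the actor.
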(event `self.ReceiveBeginPlay`
  (`parent.ReceiveBeginPlay`))

(event `self.ReceiveTick`
  (params (DeltaSeconds :type "Float (single-precision)"))
  (bind _output_get (set `self.DeltaTime` DeltaSeconds))
  (`parent.ReceiveTick` _output_get)
  (bind _returnvalue (`self.GetSkillData`))
  (switch `ESkillActorLifeCycleStep` (`self.CurrentStep`)
    (:`DelayTime`
      (`self.LinearTransformInDuration` (0.0 0.0 100.0) (`.SkillDelayTime` (break `BossSkillData` _returnvalue))))))

(event `self.CustomSkillOperation`
  (params (EffectSequence :type Integer) (TargetActor :type "Actor Object Reference") (SkillData :type "CurEffectIndexSkillData Structure") (SkillActor :type "Actor Object Reference"))
  (bind _asbp_peppy (cast `/Game/Blueprints/Actors/BP_Peppy` (`GameplayStatics.GetPlayerCharacter` 0)))
  (`PeppyStatComponent.GetDamaged` (`Peppy.StatComponent` _asbp_peppy) (`.Value_N` (break `CurEffectIndexSkillData` SkillData)))
  (`self.K2_DestroyActor`))

(fn `LinearTransformInDuration`
  (params (Movement :type "Vector Structure") (Duration :type "Float (double-precision)"))
  (`self.GetSkillData`)
  (`SceneComponent.K2_AddRelativeLocation` (`self.SkillMeshPivot`) (* Movement (/ (`self.DeltaTime`) Duration)) false false))

(fn `UserConstructionScript`
  (`parent.UserConstructionScript`))