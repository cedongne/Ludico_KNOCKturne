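; Episode 1 boss skill actor for a BindPeppy unit, animating its mesh through the skill's timed steps.
; During Delay Time, Tick raises the mesh pivot by a fixed height spread over the skill's delay time.
; During Cast Time, a DoOnce picks one of three preset rotations at random, which is applied gradually over the cast time.
; Both motions are delta-time-scaled increments, with step state and lifecycle left to the parent class.
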(event `self.ReceiveBeginPlay`
  (`parent.ReceiveBeginPlay`))

(event `self.ReceiveTick`
  (params (DeltaSeconds :type "Float (single-precision)"))
  (bind _output_get (set `self.DeltaTime` DeltaSeconds))
  (`parent.ReceiveTick` _output_get)
  (bind _returnvalue (`self.GetSkillData`))
  (switch `ESkillActorLifeCycleStep` (`self.CurrentStep`)
    (:`DelayTime`
      (bind (_bossskillid _skillstance _skillcoolturn _sprayenergy _skilldelaytime _skillcasttime) (break `BossSkillData` _returnvalue))
      (`self.LinearTransformInDuration_Loc` (0.0 0.0 480.0) _skilldelaytime))
    (:`CastTime`
      (`|ExecutionSequence`
        (:`then_0`
          (`/Engine/EditorBlueprintResources/StandardMacros.DoOnce` false
            (:`Completed`
              (set `self.Random Rotation` (`|GetArrayItem` (`self.Skill Rotations`) (`KismetMathLibrary.RandomInteger` 3))))))
        (:`then_1`
          (`self.LinearTransformInDuration_Rot` (`self.Random Rotation`) _skillcasttime))))))

(fn `LinearTransformInDuration_Loc`
  (params (Movement :type "Vector Structure") (Duration :type "Float (double-precision)"))
  (`self.GetSkillData`)
  (`SceneComponent.K2_AddRelativeLocation` (`self.SkillMeshPivot`) (* Movement (/ (`self.DeltaTime`) Duration)) false false))

(fn `LinearTransformInDuration_Rot`
  (params (`Rotate Degree` :type "Rotator Structure") (Duration :type "Float (double-precision)"))
  (`self.GetSkillData`)
  (`SceneComponent.K2_AddRelativeRotation` (`self.SkillMesh`) (* `Rotate Degree` (/ (`self.DeltaTime`) Duration)) false false))

(fn `UserConstructionScript`
  (`parent.UserConstructionScript`))