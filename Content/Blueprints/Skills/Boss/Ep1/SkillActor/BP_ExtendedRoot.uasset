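; Episode 1 boss skill actor for Extended Root, handling the skill's visual effect on top of its parent skill actor logic.
; Tick switches on the inherited CurrentStep, using DoOnce nodes so each step's action fires a single time.
; Cast Time spawns a BossHitEffectActor at a fixed world location and assigns it the NS_ExtendedRoot Niagara system.
; Destroy Time destroys that effect actor.
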(event `self.ReceiveBeginPlay`
  (`parent.ReceiveBeginPlay`))

(event `self.ReceiveTick`
  (params (DeltaSeconds :type "Float (single-precision)"))
  (bind _output_get (set `self.DeltaTime` DeltaSeconds))
  (`parent.ReceiveTick` _output_get)
  (bind _returnvalue (`self.GetSkillData`))
  (switch `ESkillActorLifeCycleStep` (`self.CurrentStep`)
    (:`CastTime`
      (`/Engine/EditorBlueprintResources/StandardMacros.DoOnce` false
        (:`Completed`
          (bind _returnvalue_2 (`|SpawnActorFromClass` "/Script/KNOCKturne.BossHitEffectActor" (`KismetMathLibrary.MakeTransform` (1600.0 760.0 0.0)) "Undefined" "OverrideRootScale"))
          (`NiagaraComponent.SetAsset` (`BossHitEffectActor.BossHitEffect` _returnvalue_2) "/Game/Assets/Effects/BossEffect/NS_ExtendedRoot.NS_ExtendedRoot" true))))
    (:`DestroyTime`
      (`/Engine/EditorBlueprintResources/StandardMacros.DoOnce` false
        (:`Completed`
          (`self.K2_DestroyActor` _returnvalue_2))))))

(fn `UserConstructionScript`
  (`parent.UserConstructionScript`))