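; Boss skill actor for Thorn of Love and Hatred in Ep1: a unit that rises, then periodically fires thorn projectiles, with a sound event on spawn.
; During the delay step it moves SkillMesh upward linearly over the skill's delay time; despite its name, RotateDegree is a location offset.
; During the cast step, a one-second delta-time timer spawns Thorn actors above the pivot, randomly using triangle or inverted-triangle rotation sets.
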(event `self.ReceiveBeginPlay`
  (`AkGameplayStatics.PostEvent` "/Game/Assets/Sounds/Wwise/Battle/ThornOfLove.ThornOfLove" (`GameplayStatics.GetGameMode`))
  (`parent.ReceiveBeginPlay`))

(event `self.ReceiveTick`
  (params (DeltaSeconds :type "Float (single-precision)"))
  (bind _output_get (set `self.DeltaTime` DeltaSeconds))
  (`parent.ReceiveTick` _output_get)
  (bind _returnvalue (`self.GetSkillData`))
  (switch `ESkillActorLifeCycleStep` (`self.CurrentStep`)
    (:`DelayTime`
      (`self.LinearTransformInDuration` (0.0 0.0 300.0) (`.SkillDelayTime` (break `BossSkillData` _returnvalue)) (`self.SkillMesh`)))
    (:`CastTime`
      (bind _returnvalue_2 (`self.DelayWithDeltaTime` 1.0 (`self.DeltaTime`)))
      (if _returnvalue_2
        (`self.ShootFlowerPeriodic`)))))

(fn `LinearTransformInDuration`
  (params (RotateDegree :type "Vector Structure") (Duration :type "Float (double-precision)") (TargetComponent :type "SceneComponent Object Reference"))
  (`self.GetSkillData`)
  (`SceneComponent.K2_AddRelativeLocation` TargetComponent (* RotateDegree (/ (`self.DeltaTime`) Duration)) false false))

(fn `ShootFlowerPeriodic`
  (bind _returnvalue (+ (`SceneComponent.K2_GetComponentLocation` (`self.ActorPivot`)) (0.0 0.0 30.0)))
  (if (`KismetMathLibrary.RandomBool`)
    (for _array_element (`self.SpawnRotations`)
      (`|SpawnActorFromClass` "/Game/Blueprints/Skills/Boss/Ep1/SkillActor/BP_ThornOfLoveAndHatred_Thorn.BP_ThornOfLoveAndHatred_Thorn_C" (`KismetMathLibrary.MakeTransform` _returnvalue _array_element) "Undefined" "OverrideRootScale" null null))
    (else
      (for _array_element_2 (`self.ReverseSpawnRotations`)
        (`|SpawnActorFromClass` "/Game/Blueprints/Skills/Boss/Ep1/SkillActor/BP_ThornOfLoveAndHatred_Thorn.BP_ThornOfLoveAndHatred_Thorn_C" (`KismetMathLibrary.MakeTransform` _returnvalue _array_element_2) "Undefined" "OverrideRootScale" null null)))))

(fn `UserConstructionScript`
  (`parent.UserConstructionScript`))