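; Boss skill actor for the Ep1 Heightened Longing attack, a flower that tracks the player and damages BP_Peppy by the skill's value.
; During Delay Time it follows the player for one second with an optional hit-area preview, then stops and raises its mesh pivot each tick.
; Cast Time shows the black attack range, and a timer holds off CanDestroy until the flower has been up for ten seconds.
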(event `self.ReceiveBeginPlay`
  (`AkGameplayStatics.PostEvent` "/Game/Assets/Sounds/Wwise/Peppy/BS_HeightenedLonging.BS_HeightenedLonging" (`GameplayStatics.GetGameMode`))
  (`parent.ReceiveBeginPlay`))

(event `self.ReceiveTick`
  (params (DeltaSeconds :type "Float (single-precision)"))
  (bind _output_get (set `self.DeltaTime` DeltaSeconds))
  (`parent.ReceiveTick` _output_get)
  (`self.Count Flower Maintain Time`)
  (bind _returnvalue (`self.GetSkillData`))
  (switch `ESkillActorLifeCycleStep` (`self.CurrentStep`)
    (:`DelayTime`
      (bind _output_get_2 (set `self.Flower Follow Time` (+ (`self.DeltaTime`) (`self.Flower Follow Time`))))
      (if (<= _output_get_2 1.0)
        (`self.SetAttackRangeForSkillVis`)
        (`self.Follow Player`)
        (else
          (`SceneComponent.SetVisibility` (`self.AttackRangeForSkill`) false false)
          ;[1 0.2917 0.2917] 모델링 변경 후 Movement 변경 필요
          (`self.LinearTransformInDuration` (0.0 0.0 200.0) 1.0)
          (set `self.Is Flower Up` true)
          (set `self.CanDestroy` false))))
    (:`CastTime`
      (`SceneComponent.SetVisibility` (`self.BlackAttackRange`) true false))))

(event `self.CustomSkillOperation`
  (params (EffectSequence :type Integer) (TargetActor :type "Actor Object Reference") (SkillData :type "CurEffectIndexSkillData Structure") (SkillActor :type "Actor Object Reference"))
  (bind _asbp_peppy (cast `/Game/Blueprints/Actors/BP_Peppy` (`GameplayStatics.GetPlayerCharacter` 0)))
  (`PeppyStatComponent.GetDamaged` (`Peppy.StatComponent` _asbp_peppy) (`.Value_N` (break `CurEffectIndexSkillData` SkillData))))

(fn `Count Flower Maintain Time`
  (if (`self.Is Flower Up`)
    (if (>= (`self.Flower Maintain Time`) 10.0)
      (set `self.CanDestroy` true)
      (else
        (set `self.Flower Maintain Time` (+ (`self.DeltaTime`) (`self.Flower Maintain Time`)))))))

(fn `Follow Player`
  (`self.K2_SetActorLocation` (`self.K2_GetActorLocation` (`GameplayStatics.GetPlayerPawn` 0))))

(fn `LinearTransformInDuration`
  (params (Movement :type "Vector Structure") (Duration :type "Float (double-precision)"))
  (`self.GetSkillData`)
  (`SceneComponent.K2_AddRelativeLocation` (`self.SkillMeshPivot`) (* Movement (/ (`self.DeltaTime`) Duration)) false false))

(fn `SetAttackRangeForSkillVis`
  (bind _returnvalue (`GameplayStatics.GetActorOfClass` "/Game/Blueprints/Actors/Battle/BP_BattleFoothold.BP_BattleFoothold_C"))
  (`/Engine/EditorBlueprintResources/StandardMacros.IsValid` _returnvalue
    (:`Is Valid`
      (if (`BattleManagerSystem.VisibleBossSkillHitArea` (subsystem `BattleManagerSystem`))
        (`SceneComponent.SetVisibility` (`self.AttackRangeForSkill`) true false)
        (else
          (`SceneComponent.SetVisibility` (`self.AttackRangeForSkill`) false false))))))

(fn `UserConstructionScript`
  (`parent.UserConstructionScript`))