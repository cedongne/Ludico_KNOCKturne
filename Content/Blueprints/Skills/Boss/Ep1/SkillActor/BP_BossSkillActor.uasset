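; Base-style actor for a boss skill, handling its attack range display and delayed animation start.
; On BeginPlay it initializes and registers AttackRange with the battle manager's hit-area list, showing it according to the VisibleBossSkillHitArea flag.
; StartSkillAnimationAfterSkillDelayTime refreshes that visibility, waits the skill data's delay plus a pre-spawn range display time, then unpauses the supplied animation.
; HitVisualEffect is an empty stub.
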(event `self.ReceiveBeginPlay`
  (`self.Initialize`)
  (`self.InitAttackRangeSetting`))

(event `StartSkillAnimationAfterSkillDelayTime`
  (params (NewParam :type "SkeletalMeshComponent Object Reference"))
  (`SceneComponent.SetHiddenInGame` (`self.AttackRange`) (not (`BattleManagerSystem.VisibleBossSkillHitArea` (subsystem `BattleManagerSystem`))) false)
  (bind _returnvalue (`self.GetSkillData`))
  (`KismetSystemLibrary.Delay` (+ (`.SkillDelayTime` (break `BossSkillData` _returnvalue)) (`self.ShowAttackRangeTime_PreSpawnActor`)))
  (`self.PlaySkillAnimation` NewParam))

(fn `HitVisualEffect`)

(fn `InitAttackRangeSetting`
  (bind _returnvalue (subsystem `BattleManagerSystem`))
  (bind _attackrange (`self.AttackRange`))
  (`KismetArrayLibrary.Array_Add` (`BattleManagerSystem.CurBossSkillHitArea` _returnvalue) _attackrange)
  (`SceneComponent.SetHiddenInGame` _attackrange (not (`BattleManagerSystem.VisibleBossSkillHitArea` _returnvalue)) false))

(fn `PlaySkillAnimation`
  (params (SkillAnimation :type "SkeletalMeshComponent Object Reference"))
  (set `SkeletalMeshComponent.bPauseAnims` false SkillAnimation))

(fn `UserConstructionScript`)