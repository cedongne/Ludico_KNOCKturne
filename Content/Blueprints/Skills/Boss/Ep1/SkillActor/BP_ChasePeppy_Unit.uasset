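; Episode 1 boss skill unit for a "ChasePeppy" attack, driven by the skill step and data.
; During Delay Time it raises its mesh pivot 500 units over the skill's delay.
; During Cast Time ChsaePlayer moves it by Speed along the player-to-unit direction, which points away from the player unless Speed is negative.
; Overlapping player 0 destroys every unit of this class, with no damage applied here.
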(event `self.ReceiveBeginPlay`
  (`parent.ReceiveBeginPlay`))

(event `self.ReceiveActorBeginOverlap`
  (params (OtherActor :type "Actor Object Reference"))
  (if (== OtherActor (`GameplayStatics.GetPlayerCharacter` 0))
    (bind _outactors (`GameplayStatics.GetAllActorsOfClass` "BP_ChasePeppy_Unit_C"))
    (for _array_element _outactors
      (`self.K2_DestroyActor` _array_element))))

(event `self.ReceiveTick`
  (params (DeltaSeconds :type "Float (single-precision)"))
  (bind _output_get (set `self.DeltaTime` DeltaSeconds))
  (`parent.ReceiveTick` _output_get)
  (bind _returnvalue (`self.GetSkillData`))
  (switch `ESkillActorLifeCycleStep` (`self.CurrentStep`)
    (:`DelayTime`
      (`self.LinearTransformInDuration` (0.0 0.0 500.0) (`.SkillDelayTime` (break `BossSkillData` _returnvalue))))
    (:`CastTime`
      (`self.Chsae Player`))))

(fn `Chsae Player`
  (locals (Movement :type "Vector Structure") (Speed :type "Float (double-precision)" :default 5.0) (Velocity :type "Vector Structure"))
  (bind _output_get (set `local.Movement` (`KismetMathLibrary.Normal` (- (`self.K2_GetActorLocation`) (`self.K2_GetActorLocation` (`GameplayStatics.GetPlayerCharacter` 0))))))
  (bind _output_get_2 (set `local.Velocity` (* (* _output_get (`local.Speed`)) (`self.DeltaTime`))))
  (`self.K2_SetActorLocation` (+ (`self.K2_GetActorLocation`) _output_get_2)))

(fn `LinearTransformInDuration`
  (params (Movement :type "Vector Structure") (Duration :type "Float (double-precision)"))
  (`self.GetSkillData`)
  (`SceneComponent.K2_AddRelativeLocation` (`self.SkillMeshPivot`) (* Movement (/ (`self.DeltaTime`) Duration)) false false))

(fn `UserConstructionScript`
  (`parent.UserConstructionScript`))