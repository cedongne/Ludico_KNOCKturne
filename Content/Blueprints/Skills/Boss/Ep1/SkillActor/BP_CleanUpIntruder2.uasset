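; Skill actor for an Episode 1 boss's "Clean Up Intruder 2" skill that animates the rotation of its mesh pivot.
; Each tick runs the parent logic, then rotates the pivot on one axis during the delay step and another during the cast step.
; Rotation is scaled by delta time over that step's duration from skill data, spreading a fixed angle across it.
; TransformInCastTime is unused and divides by delay time despite its name.
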(event `self.ReceiveBeginPlay`
  (`parent.ReceiveBeginPlay`))

(event `self.ReceiveTick`
  (params (DeltaSeconds :type "Float (single-precision)"))
  (bind _output_get (set `self.DeltaTime` DeltaSeconds))
  (`parent.ReceiveTick` _output_get)
  (bind _returnvalue (`self.GetSkillData`))
  (switch `ESkillActorLifeCycleStep` (`self.CurrentStep`)
    (:`DelayTime`
      (bind (_bossskillid _skillstance _skillcoolturn _sprayenergy _skilldelaytime _skillcasttime) (break `BossSkillData` _returnvalue))
      (`self.LinearTransformInDuration` (struct :`Roll` 90.0) _skilldelaytime))
    (:`CastTime`
      (`self.LinearTransformInDuration` (struct :`Yaw` 180.0) _skillcasttime))))

(fn `LinearTransformInDuration`
  (params (RotateDegree :type "Rotator Structure") (Duration :type "Float (double-precision)"))
  (`self.GetSkillData`)
  (`SceneComponent.K2_AddRelativeRotation` (`self.SkillMeshPivot`) (* RotateDegree (/ (`self.DeltaTime`) Duration)) false false))

(fn `TransformInCastTime`
  (params (RotateDegree :type "Rotator Structure"))
  (locals (NewLocalVar_0 :type Boolean))
  (bind _returnvalue (`self.GetSkillData`))
  (`SceneComponent.K2_AddRelativeRotation` (`self.SkillMeshPivot`) (* RotateDegree (/ (`self.DeltaTime`) (`.SkillDelayTime` (break `BossSkillData` _returnvalue)))) false false))

(fn `UserConstructionScript`
  (`parent.UserConstructionScript`))