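; BP_ThornOfLoveAndHatred is an Ep1 boss skill actor that scatters several thorn unit actors across a fixed area when it begins play.
; It first generates transforms from random points in a hardcoded flat box with random yaw, retrying any point that BattleUtilManager reports as too close to those already chosen.
; It then spawns a BP_ThornOfLoveAndHatred_Unit at each stored transform.
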(event `self.ReceiveBeginPlay`
  (for _ (range 3)
    (bind _skilltansform (`self.SetRandomSkillTransform`))
    (`KismetArrayLibrary.Array_Add` (`self.SkillTransforms`) _skilltansform))
  (for _array_element (`self.SkillTransforms`)
    (`|SpawnActorFromClass` "/Game/Blueprints/Skills/Boss/Ep1/SkillActor/BP_ThornOfLoveAndHatred_Unit.BP_ThornOfLoveAndHatred_Unit_C" _array_element "Undefined" "OverrideRootScale" null null)))

(fn `SetRandomSkillTransform`
  (returns (SkillTansform :type "Transform Structure"))
  (locals (Index :type Integer))
  (bind _output_get (set `self.IsOverlap` true))
  (while _output_get
    (bind _output_get_2 (set `self.CurrentIndexLocation` (`KismetMathLibrary.RandomPointInBoundingBox` (751.0 774.0 -87.0) (400.0 400.0 0.0))))
    (bind _returnvalue (`BattleUtilManager.IsOverlappedAnotherSkills` (subsystem `BattleUtilManager`) _output_get_2 (`self.SkillTransforms`) 300))
    (set `self.IsOverlap` _returnvalue))
  (return (`KismetMathLibrary.MakeTransform` (`self.CurrentIndexLocation`) (`KismetMathLibrary.MakeRotator` 0.0 0.0 (`KismetMathLibrary.RandomFloatInRange` 0.0 360.0)))))

(fn `UserConstructionScript`)