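; BP_SweptGardenUnit is an Episode 1 boss skill actor that damages the player character Peppy on overlap.
; The first overlap with Peppy latches a one-hit flag, even if the unit is not yet initialized.
; If it is initialized, it calls HitPlayer, prints the damage value from SkillData and subtracts it directly from Peppy's current HP, truncating the result.
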(event `self.ReceiveBeginPlay`)

(event `self.ReceiveActorBeginOverlap`
  (params (OtherActor :type "Actor Object Reference"))
  (bind (_bossskillid _skillstance _skillcoolturn _sprayenergy _skilldelaytime _skillcasttime _objectspeed _skillindex_1 _probability_1 _skilltarget_1 _value_1_n) (break `BossSkillData` (`self.SkillData`)))
  (bind _aspeppy (cast `Peppy` OtherActor))
  (if (not (`self.IsHitPlayer`))
    (set `self.IsHitPlayer` true)
    (if (`self.IsInitialized`)
      (`self.HitPlayer`)
      (`KismetSystemLibrary.PrintString` (`KismetStringLibrary.Conv_DoubleToString` _value_1_n))
      (bind _peppystat (`Peppy.PeppyStat` _aspeppy))
      (set `PeppyStatComponent.CurrentHP` (`KismetMathLibrary.FTrunc` (- (`PeppyStatComponent.CurrentHP` _peppystat) _value_1_n)) _peppystat))))

(fn `UserConstructionScript`)