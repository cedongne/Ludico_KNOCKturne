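; Boss skill actor that runs a timed lifecycle for a skill and its AttackRange hit area.
; StartSkillActorLifeCycle shows or hides AttackRange according to the battle manager's VisibleBossSkillHitArea flag, then waits briefly.
; PlaySkillAnimation then unpauses animation on the passed-in object and destroys AttackRange.
; The actor destroys itself after the cast time from SkillData elapses.
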(event `StartSkillActorLifeCycle`
  (params (NewParam :type "SkeletalMeshComponent Object Reference"))
  (`SceneComponent.SetHiddenInGame` (`self.AttackRange`) (not (`BattleManagerSystem.VisibleBossSkillHitArea` (subsystem `BattleManagerSystem`))) false)
  (`KismetSystemLibrary.Delay` 1.0)
  (`self.PlaySkillAnimation` NewParam)
  (`KismetSystemLibrary.Delay` (`.SkillCastTime` (break `BossSkillData` (`self.SkillData`))))
  (`self.K2_DestroyActor`))

(fn `PlaySkillAnimation`
  (params (SkillAnimation :type "SkeletalMeshComponent Object Reference"))
  (set `SkeletalMeshComponent.bPauseAnims` false SkillAnimation)
  (`ActorComponent.K2_DestroyComponent` (`self.AttackRange`)))

(fn `UserConstructionScript`)